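; Audio visualizer Blueprint that plays a randomly selected track and drives the scale of visualization shape actors from its loudness.
; Init gathers and shuffles all Audio_Visualization_Shape_BP actors and picks a track from TracksList.
; During playback, each playback-percent callback reads the cooked envelope amplitude and passes it to every shape.
; Reset fades out the audio, resets shape scales and optionally picks another random track.
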(event `reset`
  (params (`select another track` :type Boolean))
  (`self.handle fade out` 0.5)
  (for _array_element (`self.sfx meshes`)
    (`/Game/Blueprints/World_Cube/Shape/Audio_Visualization_Shape_BP.reset scale` _array_element))
  (if `select another track`
    (`self.select a track`)))

(event `init visualizer`
  (`self.get meshes`)
  (`self.select a track`))

(event `play track`
  (bind _output_track (break `/Game/DataTypes/Audio/Track_Data_Structure` (`|GetArrayItem` (`self.tracks list`) (`self.selected index`))))
  (`|ExecutionSequence`
    (:`then_0`
      (`AudioComponent.SetSound` (`self.Audio`) _output_track))
    (:`then_1`
      (add `AudioComponent.OnAudioPlaybackPercent` (`self.Audio`) (delegate `handle playback change`))
      (`AudioComponent.Play` (`self.Audio`) 0.0))))

(event `handle playback change`
  (params (PlayingSoundWave :type "SoundWave Object Reference") (PlaybackPercent :type "Float (single-precision)"))
  (bind _outenvelopedata (`AudioComponent.GetCookedEnvelopeData` (`self.Audio`)))
  (bind _output_get (set `self.new amplitude` _outenvelopedata))
  (`self.update scale of sfx meshes` _output_get))

(event `self.Audio.OnAudioFinished`
  ;[1 1 1] it is important otherwise new amplitude will be updated
  (clear `AudioComponent.OnAudioPlaybackPercent` (`self.Audio`))
  (`KismetSystemLibrary.Delay` 1.0)
  (set `self.new amplitude` 0.0))

(event `handle fade out`
  (params (duration :type "Float (double-precision)"))
  (`AudioComponent.FadeOut` (`self.Audio`) duration 0.0 "Linear")
  (`KismetSystemLibrary.Delay` duration)
  (`AudioComponent.Stop` (`self.Audio`)))

(fn `get meshes`
  (`KismetArrayLibrary.Array_Clear` (`self.sfx meshes`))
  (bind _outactors (`GameplayStatics.GetAllActorsOfClass` "/Game/Blueprints/World_Cube/Shape/Audio_Visualization_Shape_BP.Audio_Visualization_Shape_BP_C"))
  (bind _output_get (set `self.sfx meshes` _outactors))
  (`KismetArrayLibrary.Array_Shuffle` _output_get))

(fn `select a track`
  (set `self.selected index` (`KismetMathLibrary.RandomIntegerInRange` 0 (- (`KismetArrayLibrary.Array_Length` (`self.tracks list`)) 1))))

(fn `update scale of sfx meshes`
  (params (`new amplitude` :type "Float (double-precision)"))
  (for _array_element (`self.sfx meshes`)
    (`/Game/Blueprints/World_Cube/Shape/Audio_Visualization_Shape_BP.current amplitude` _array_element (`local.new amplitude`))))

(fn `UserConstructionScript`)