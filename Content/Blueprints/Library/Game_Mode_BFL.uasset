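; Blueprint function library that supplies static lookup data for the game's three game modes.
; Each function clears and refills a map on every call, keyed by what appear to be game mode enum values.
; The functions return a name-to-context map, the background UI material for a given mode name, and a map of assignment texts describing each mode's objective and end condition.
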(fn `get game mode name to background image`
  (params (`name enum` :type "/Game/DataTypes/UI/Game_Mode_Name_ENUM Enum" :default "NewEnumerator0"))
  (returns (`return image` :type "Material Object Reference"))
  (locals (`name to image map` :type "Map of /Game/DataTypes/UI/Game_Mode_Name_ENUM Enum to Material Object Reference"))
  (`|ExecutionSequence`
    (:`then_0`
      (`BlueprintMapLibrary.Map_Clear` (`local.name to image map`))
      (`BlueprintMapLibrary.Map_Add` (`local.name to image map`) "NewEnumerator0" "/Game/My_Textures/art/Rhythm_Rush_Background_UI_Material.Rhythm_Rush_Background_UI_Material")
      (`BlueprintMapLibrary.Map_Add` (`local.name to image map`) "NewEnumerator1" "/Game/My_Textures/art/Limiting_Vibes_UI_Material.Limiting_Vibes_UI_Material")
      (`BlueprintMapLibrary.Map_Add` (`local.name to image map`) "NewEnumerator2" "/Game/My_Textures/art/Mixer_Background_UI_Material.Mixer_Background_UI_Material"))
    (:`then_1`
      (return (`BlueprintMapLibrary.Map_Find` (`local.name to image map`) (`local.name enum`))))))

(fn `get game mode name to context map`
  (returns (`return game mode name context map` :type "Map of /Game/DataTypes/UI/Game_Mode_Name_ENUM Enum to /Game/DataTypes/UI/Game_Mode_Context_ENUM Enum"))
  (locals (`game mode name context map` :type "Map of /Game/DataTypes/UI/Game_Mode_Name_ENUM Enum to /Game/DataTypes/UI/Game_Mode_Context_ENUM Enum"))
  (`|ExecutionSequence`
    (:`then_0`
      (`BlueprintMapLibrary.Map_Clear` (`local.game mode name context map`))
      (`BlueprintMapLibrary.Map_Add` (`local.game mode name context map`) "NewEnumerator0" "NewEnumerator0")
      (`BlueprintMapLibrary.Map_Add` (`local.game mode name context map`) "NewEnumerator1" "NewEnumerator1")
      (`BlueprintMapLibrary.Map_Add` (`local.game mode name context map`) "NewEnumerator2" "NewEnumerator2"))
    (:`then_1`
      (return (`local.game mode name context map`)))))

(fn `get game mode to assignment map`
  (returns (`game mode to assignment map` :type "Map of /Game/DataTypes/UI/Game_Mode_Name_ENUM Enum to String"))
  (locals (map :type "Map of /Game/DataTypes/UI/Game_Mode_Name_ENUM Enum to String"))
  (`|ExecutionSequence`
    (:`then_0`
      (`BlueprintMapLibrary.Map_Clear` (`local.map`))
      (`BlueprintMapLibrary.Map_Add` (`local.map`) "NewEnumerator0" "Defeat entities until timer runs out.")
      (`BlueprintMapLibrary.Map_Add` (`local.map`) "NewEnumerator1" "Defeat entities until quantum spheroids runs out.")
      (`BlueprintMapLibrary.Map_Add` (`local.map`) "NewEnumerator2" "Defeat entities until timer or quantum spheroids runs out."))
    (:`then_1`
      (return (`local.map`)))))