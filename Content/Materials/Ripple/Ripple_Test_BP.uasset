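; Test actor that drives a ripple material effect on a Plane mesh.
; The construction script creates a dynamic instance of Ripple_Material_Instance and assigns it to the Plane's first slot, redundantly across three sequence pins.
; On BeginPlay it sets the material's center to the actor's location, then plays a timeline that feeds the radius parameter on the Plane's materials.
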(event `self.ReceiveBeginPlay`
  (`MaterialInstanceDynamic.SetVectorParameterValue` (`self.dm`) "center" (`KismetMathLibrary.Conv_VectorToLinearColor` (`self.K2_GetActorLocation`)))
  (bind (_direction _newtrack_0) (`Timeline|Timeline`)
    (:`Update`
      (`MeshComponent.SetScalarParameterValueOnMaterials` (`self.Plane`) "radius" _newtrack_0))))

(fn `UserConstructionScript`
  (bind _plane (`self.Plane`))
  (bind _returnvalue (`KismetMaterialLibrary.CreateDynamicMaterialInstance` "/Game/Materials/Ripple/Ripple_Material_Instance.Ripple_Material_Instance"))
  (bind _output_get (set `self.dm` _returnvalue))
  (`|ExecutionSequence`
    (:`then_0`
      (`PrimitiveComponent.SetMaterial` _plane 0 _output_get))
    (:`then_1`
      (`PrimitiveComponent.SetMaterial` _plane 0 (`self.dm`)))
    (:`then_2`
      (`PrimitiveComponent.SetMaterial` _plane 0 (`self.dm`)))))