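; Floor shape Blueprint in the World_Cube folder that gives itself a random size when play begins.
; BeginPlay sets the root component's relative scale from MakeRandomVector, which rolls each axis independently between one and three, so scaling is usually non-uniform.
; MakeRandomVector also holds unreachable leftover logic for randomizing only axes flagged by a Scalar vector.
; The construction script is empty.
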(event `self.ReceiveBeginPlay`
  (`SceneComponent.SetRelativeScale3D` (`self.DefaultSceneRoot`) (`self.make random vector` 1.0 3.0)))

(fn `make random vector`
  (params (min :type "Float (double-precision)" :default 1.0) (max :type "Float (double-precision)" :default 10.0))
  (returns (`random vector` :type "Vector Structure"))
  (locals (final :type "Vector Structure" :default (1.0 1.0 1.0)))
  (return (`KismetMathLibrary.MakeVector` (`KismetMathLibrary.RandomFloatInRange` (`local.min`) (`local.max`)) (`KismetMathLibrary.RandomFloatInRange` (`local.min`) (`local.max`)) (`KismetMathLibrary.RandomFloatInRange` (`local.min`) (`local.max`)))))

(fn `UserConstructionScript`)