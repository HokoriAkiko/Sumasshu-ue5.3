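; Enemy obstacle Blueprint that reacts to projectile hits and blasts, extending its parent's hit and kill handling.
; Each hit calls the parent, spawns a status popup at the collider labelled with a fixed physical or explosive text, then activates a Niagara effect.
; The projectile's element name is passed to the parent but does not affect the popup text.
; On kill, it runs the parent logic and destroys the actor.
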(event `/Game/Blueprints/Interface/Ball_Projectile_On_Hit_BPI.hit by projectile`
  (params (`damage configuration` :type "/Game/DataTypes/Projectile_Damage_Configuration_Data_Structure Structure") (`projectile element name` :type "String (by ref)"))
  (`parent.hit by projectile` `damage configuration` `projectile element name`)
  (`self.handle spawning of vfx` "Physical Bolt")
  (bind _niagara (`self.Niagara` :!label _label)
    (:`then`
      (`ActorComponent.Activate` _niagara true))
    (:`else`)))

(event `/Game/Blueprints/Interface/Kill_BPI.handle kill`
  (`parent.handle kill`)
  (`self.K2_DestroyActor`))

(event `/Game/Blueprints/Interface/Blast_BPI.hit by blast`
  (params (`blast configuration` :type "/Game/DataTypes/Blast_Damage_Configuration_Data_Structure Structure"))
  (`parent.hit by blast` `blast configuration`)
  (`self.handle spawning of vfx` "Explosive Impact")
  (goto _label))

(fn `handle spawning of vfx`
  (params (status :type Text :default "NSLOCTEXT(\"[B3F25551AD28237B30CDECEA55D90B24]\", \"E325642E40013D0695132F9274F7D5BD\", \"Default Text\")"))
  (`|ExecutionSequence`
    (:`then_0`
      (if (!= (`KismetStringLibrary.Len` (`KismetTextLibrary.Conv_TextToString` (`local.status`))) 0)
        (bind _collider (`self.collider`)
          (:`then`
            (`|SpawnActorFromClass` "/Game/Blueprints/Hit_Status_Popup_BP.Hit_Status_Popup_BP_C" (`KismetMathLibrary.MakeTransform` (`SceneComponent.K2_GetComponentLocation` _collider)) "Undefined" "MultiplyWithRoot" null (`local.status`) null))
          (:`else`))))))

(fn `UserConstructionScript`)