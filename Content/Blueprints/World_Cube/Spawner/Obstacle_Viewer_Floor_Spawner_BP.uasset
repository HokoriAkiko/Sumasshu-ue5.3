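; Spawner actor that builds a square floor of Floor_Shape_BP tiles, by its name for an obstacle viewer.
; On BeginPlay, nested loops spawn an 11 by 11 grid centered on zero, with MakeLocationVector turning indices into evenly spaced offsets, X negated.
; Each tile attaches to the root with KeepRelative rules, so those offsets become relative to the spawner.
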(event `self.ReceiveBeginPlay`
  (for _index (range -5 6)
    (for _index_2 (range -5 6)
      (bind _returnvalue (`|SpawnActorFromClass` "/Game/Blueprints/World_Cube/Shape/Floor_Shape_BP.Floor_Shape_BP_C" (`KismetMathLibrary.MakeTransform` (`self.make location vector` _index_2 _index)) "Undefined" "MultiplyWithRoot" null (0.0 0.0 1.0) null))
      (`self.K2_AttachToComponent` _returnvalue (`self.DefaultSceneRoot`) "None" "KeepRelative" "KeepRelative" "KeepRelative" true))))

(fn `make location vector`
  (params (`x index` :type Integer) (`y index` :type Integer))
  (returns (`return vector` :type "Vector Structure"))
  (return (`KismetMathLibrary.MakeVector` (`KismetMathLibrary.Conv_IntToDouble` (* `x index` -200)) (`KismetMathLibrary.Conv_IntToDouble` (* `y index` 200)))))

(fn `UserConstructionScript`)