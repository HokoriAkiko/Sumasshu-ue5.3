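; Helper Blueprint function library with a SortByElement function that returns an array's elements in ascending order.
; It uses a selection sort: each pass scans a working array for the index of the minimum, appends that value to the sorted array and removes it from the working one.
; The outer loop is an execution wire looped back to the length check, repeating until the working array is empty.
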(fn `sort by element`
  (params (arr :type "Array of Integer"))
  (returns (`return sorted` :type "Array of Integer"))
  (locals (`sorted arr` :type "Array of Integer") (`min index` :type Integer :default 0) (`temp arr` :type "Array of Integer"))
  (bind _temp_arr (`local.temp arr`))
  (bind _output_get (set `local.temp arr` arr))
  (if (!= (`KismetArrayLibrary.Array_Length` _output_get) 0) :!label _label
    ;[1 1 1] finding min value using index
    (for (_array_element _array_index) _temp_arr
      (if (< _array_element (`|GetArrayItem` _temp_arr (`local.min index`)))
        (set `local.min index` _array_index)))
    ;[1 1 1] pushing min value to sorted array
    (`KismetArrayLibrary.Array_Add` (`local.sorted arr`) (`|GetArrayItem` (`local.temp arr`) (`local.min index`)))
    ;[1 1 1] deleting that min value from original array
    (`KismetArrayLibrary.Array_Remove` (`local.temp arr`) (`local.min index`))
    ;[1 1 1] resetting min index
    (set `local.min index` 0)
    (goto _label)
    (else
      (return (`local.sorted arr`)))))