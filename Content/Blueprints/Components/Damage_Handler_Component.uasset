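; Enemy damage component that resolves projectile and blast hits into HP loss, score and kill handling.
; Projectile and enemy elements are matched in either order against a reaction table built at BeginPlay, spawning a reaction, physical or immune popup.
; Reaction percentages, adjusted by the current stage's effects from level data, scale elemental damage alongside physical damage.
; Blast damage is calculated separately, but its zero multiplier cancels each contribution.
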(event `init refs`
  (`|ExecutionSequence`
    (:`then_0`
      (bind _asgameplay_gm (cast `/Game/Blueprints/Gameplay_GM` (`GameplayStatics.GetGameMode`)))
      (set `self.As Gameplay GM` _asgameplay_gm))
    (:`then_1`
      (bind _outactors (`GameplayStatics.GetAllActorsOfClass` "/Game/Blueprints/Save_Data/Level_Effect_Save_Data_BP.Level_Effect_Save_Data_BP_C"))
      (set `self.level effect ref` (`|GetArrayItem` _outactors))
      (`self.prepare index to stage effect`))
    (:`then_2`
      (bind _asenemy_base_bp (cast `/Game/Blueprints/Obstacles/Enemy/Enemy_Base_BP` (`self.GetOwner`)))
      (set `self.As Enemy Base BP` _asenemy_base_bp))))

(event `self.ReceiveBeginPlay`
  (`self.init refs`)
  (`self.make reaction info list`))

(event `handle projectile damage`
  (params (`damage configuration` :type "/Game/DataTypes/Projectile_Damage_Configuration_Data_Structure Structure") (`projectile element` :type String) (`my element` :type String))
  (bind _calculated_damage (`self.handle reaction` `damage configuration` `projectile element` `my element`))
  (`self.update scoring and hp` _calculated_damage))

(event `handle blast damage`
  (params (`blast configuration` :type "/Game/DataTypes/Blast_Damage_Configuration_Data_Structure Structure"))
  (bind _calculated_damage (`self.calculate blast damage` `blast configuration`))
  (`self.update scoring and hp` _calculated_damage))

(fn `calculate blast damage`
  (params (`blast configuration` :type "/Game/DataTypes/Blast_Damage_Configuration_Data_Structure Structure"))
  (returns (`calculated damage` :type Integer))
  (locals (final :type Integer))
  (bind (_blast_configuration_candeliverelementaldamage _blast_configuration_candeliverphysicaldamage _blast_configuration_physicaldamagevalue _blast_configuration_elementaldamagevalue _blast_configuration_physicaldamagepercent) (break `/Game/DataTypes/Blast_Damage_Configuration_Data_Structure` (`local.blast configuration`)))
  (bind (_blast_configuration_candeliverelementaldamage_2 _blast_configuration_candeliverphysicaldamage_2 _blast_configuration_physicaldamagevalue_2 _blast_configuration_elementaldamagevalue_2 _blast_configuration_physicaldamagepercent_2 _blast_configuration_elementaldamagepercent) (break `/Game/DataTypes/Blast_Damage_Configuration_Data_Structure` (`local.blast configuration`)))
  (`|ExecutionSequence`
    (:`then_0`
      (if _blast_configuration_candeliverelementaldamage_2
        (set `local.final` (`KismetMathLibrary.FTrunc` (+ (`local.final`) (* 0.01 _blast_configuration_elementaldamagevalue_2 _blast_configuration_elementaldamagepercent 0.0))))))
    (:`then_1`
      (if _blast_configuration_candeliverphysicaldamage
        (set `local.final` (`KismetMathLibrary.FTrunc` (+ (`local.final`) (* 0.01 _blast_configuration_physicaldamagevalue _blast_configuration_physicaldamagepercent 0.0))))))
    (:`then_2`
      (return (`local.final`)))))

(fn `calculate damage`
  (params (`elemental percent` :type Integer) (`reaction name` :type String) (`damage config` :type "/Game/DataTypes/Projectile_Damage_Configuration_Data_Structure Structure") (`physical percent` :type Integer))
  (returns (`calculated damage` :type Integer))
  (locals (final :type Integer))
  (bind _damage_config_physical (break `/Game/DataTypes/Projectile_Damage_Configuration_Data_Structure` (`local.damage config`)))
  (bind (_damage_config_physical_2 _damage_config_elemental) (break `/Game/DataTypes/Projectile_Damage_Configuration_Data_Structure` (`local.damage config`)))
  (bind _damage_type_config_elemental (break `/Game/DataTypes/Damage_Type_Configuration_Data_Structure` (`/Game/Blueprints/Obstacles/Enemy/Enemy_Base_BP.damage type config` (`self.As Enemy Base BP`))))
  (bind (_damage_type_config_elemental_2 _damage_type_config_physical) (break `/Game/DataTypes/Damage_Type_Configuration_Data_Structure` (`/Game/Blueprints/Obstacles/Enemy/Enemy_Base_BP.damage type config` (`self.As Enemy Base BP`))))
  (`|ExecutionSequence`
    (:`then_0`
      (if (and (`KismetStringLibrary.NotEqual_StrStr` (`local.reaction name`) "IMMUNE") _damage_type_config_elemental)
        (set `local.final` (+ (`local.final`) (* _damage_config_elemental (`self.update damage percent based on stage effect` (`local.reaction name`) (`local.elemental percent`)) 0.01)))))
    (:`then_1`
      (if _damage_type_config_physical
        (set `local.final` (+ (`local.final`) (* (`local.physical percent`) _damage_config_physical 0.01)))))
    (:`then_2`
      (return (`local.final`)))))

(fn `find and spawn reaction`
  (params (`projectile element` :type String) (`my element` :type String))
  (returns (name :type String) (`elemental percent` :type Integer) (`reaction color` :type "LinearColor Structure") (`is physical` :type Boolean) (`is immune` :type Boolean) (`physical percent` :type Integer))
  (locals (`temp index` :type Integer :default -1) (`immune reaction name color` :type "LinearColor Structure" :default (struct :`R` 0.5 :`G` 0.5 :`B` 0.5 :`A` 1.0)))
  (bind _immune_reaction_name_color (`local.immune reaction name color`))
  (bind (_output_element1 _output_element2 _output_reactionname _output_reactionpercent _output_reactioncolor) (break `/Game/DataTypes/Reaction_Info_Data_Structure` (`|GetArrayItem` (`self.reaction info list`) (`local.temp index`))))
  (bind _returnvalue (`KismetMathLibrary.Conv_ColorToLinearColor` (`/Game/Blueprints/Components/Element_Assignment_Component.selected element color` (`/Game/Blueprints/Obstacles/Enemy/Enemy_Base_BP.Element_Assignment_Component` (`self.As Enemy Base BP`)))))
  (if (or (`KismetStringLibrary.EqualEqual_StrStr` `projectile element` "NEUTRAL") (`KismetStringLibrary.EqualEqual_StrStr` `my element` "PHYSICAL"))
    (`self.handle reaction name spawning` "PHYSICAL" _returnvalue)
    (return "PHYSICAL" 0 _returnvalue true false 100)
    (else
      (`|ExecutionSequence`
        (:`then_0`
          (for (_array_element _array_index) (`self.reaction info list`)
            (if (or (and (`KismetStringLibrary.EqualEqual_StrStr` (break `/Game/DataTypes/Reaction_Info_Data_Structure` _array_element) (`local.projectile element`)) (`KismetStringLibrary.EqualEqual_StrStr` (`.element2_4_AE1CDA044E883E80DCC7E58E9565B295` (break `/Game/DataTypes/Reaction_Info_Data_Structure` _array_element)) (`local.my element`))) (and (`KismetStringLibrary.EqualEqual_StrStr` (break `/Game/DataTypes/Reaction_Info_Data_Structure` _array_element) (`local.my element`)) (`KismetStringLibrary.EqualEqual_StrStr` (`.element2_4_AE1CDA044E883E80DCC7E58E9565B295` (break `/Game/DataTypes/Reaction_Info_Data_Structure` _array_element)) (`local.projectile element`))))
              (set `local.temp index` _array_index))))
        (:`then_1`
          (if (== (`local.temp index`) -1)
            (`self.handle reaction name spawning` "IMMUNE" _immune_reaction_name_color)
            (return "Immune" 0 _immune_reaction_name_color false true 0)
            (else
              (`self.handle reaction name spawning` _output_reactionname _output_reactioncolor)
              (return _output_reactionname _output_reactionpercent _output_reactioncolor false false 0))))))))

(fn `handle reaction`
  (params (`damage configuration` :type "/Game/DataTypes/Projectile_Damage_Configuration_Data_Structure Structure") (`projectile element` :type String) (`my element` :type String))
  (returns (`calculated damage` :type Integer))
  (locals (`temp name` :type String) (`temp percent` :type Integer :default 0) (`final damage` :type Integer))
  (`|ExecutionSequence`
    (:`then_0`
      (bind (_name _elemental_percent _reaction_color _is_physical _is_immune _physical_percent) (`self.find and spawn reaction` `projectile element` `my element`))
      (set `/Game/Blueprints/Obstacles/Enemy/Enemy_Base_BP.reaction occured` (not _is_immune) (`self.As Enemy Base BP`))
      (return (`self.calculate damage` _elemental_percent _name (`local.damage configuration`) _physical_percent)))))

(fn `handle reaction name spawning`
  (params (name :type String) (`reaction color` :type "LinearColor Structure"))
  (`|SpawnActorFromClass` "/Game/Blueprints/Reaction_Name_Popup_BP.Reaction_Name_Popup_BP_C" (`KismetMathLibrary.MakeTransform` (+ (`Actor.K2_GetActorLocation` (`self.GetOwner`)) (`KismetMathLibrary.MakeVector` (`KismetMathLibrary.RandomFloatInRange` -200.0 -100.0) 0.0 (`KismetMathLibrary.RandomFloatInRange` 0.0 200.0)))) "Undefined" "MultiplyWithRoot" null (`local.name`) (`local.reaction color`) null))

(fn `make reaction info list`
  (`|ExecutionSequence`
    (:`then_0`
      ;[1 1 1] hydro based reactions
      (`KismetArrayLibrary.Array_Add` (`self.reaction info list`) (make `/Game/DataTypes/Reaction_Info_Data_Structure` "HYDRO" "GEO" "CRYSTALLIZE" 50 (struct :`R` 100.0 :`G` 100.0 :`A` 1.0)))
      (`KismetArrayLibrary.Array_Add` (`self.reaction info list`) (make `/Game/DataTypes/Reaction_Info_Data_Structure` "HYDRO" "DENDRO" "BLOOM" 100 (struct :`G` 100.0 :`A` 1.0))))
    (:`then_1`
      ;[1 1 1] anemo based reactions
      (`KismetArrayLibrary.Array_Add` (`self.reaction info list`) (make `/Game/DataTypes/Reaction_Info_Data_Structure` "ANEMO" "HYDRO" "SWIRL" 25 (struct :`G` 99.999954 :`B` 100.0 :`A` 1.0))))
    (:`then_2`
      ;[1 1 1] electro based reactions
      (`KismetArrayLibrary.Array_Add` (`self.reaction info list`) (make `/Game/DataTypes/Reaction_Info_Data_Structure` "ELECTRO" "ANEMO" "SWIRL" 25 (struct :`G` 100.0 :`B` 100.0 :`A` 1.0)))
      (`KismetArrayLibrary.Array_Add` (`self.reaction info list`) (make `/Game/DataTypes/Reaction_Info_Data_Structure` "ELECTRO" "HYDRO" "ELECTRO CHARGED" 45 (struct :`R` 50.0 :`B` 100.0 :`A` 1.0)))
      (`KismetArrayLibrary.Array_Add` (`self.reaction info list`) (make `/Game/DataTypes/Reaction_Info_Data_Structure` "ELECTRO" "GEO" "CRYSTALLIZE" 50 (struct :`R` 100.0 :`G` 100.0 :`A` 1.0)))
      (`KismetArrayLibrary.Array_Add` (`self.reaction info list`) (make `/Game/DataTypes/Reaction_Info_Data_Structure` "ELECTRO" "DENDRO" "QUICKEN" 65 (struct :`G` 100.0 :`A` 1.0))))
    (:`then_3`
      ;[1 1 1] cryo based reactions
      (`KismetArrayLibrary.Array_Add` (`self.reaction info list`) (make `/Game/DataTypes/Reaction_Info_Data_Structure` "CRYO" "ELECTRO" "SUPERCONDUCT" 45 (struct :`R` 10.000002 :`G` 10.000002 :`B` 100.0 :`A` 1.0)))
      (`KismetArrayLibrary.Array_Add` (`self.reaction info list`) (make `/Game/DataTypes/Reaction_Info_Data_Structure` "CRYO" "ANEMO" "SWIRL" 25 (struct :`R` 10.000002 :`G` 99.999962 :`B` 100.0 :`A` 1.0)))
      (`KismetArrayLibrary.Array_Add` (`self.reaction info list`) (make `/Game/DataTypes/Reaction_Info_Data_Structure` "CRYO" "HYDRO" "FROZEN" 15 (struct :`R` 50.0 :`G` 50.0 :`B` 100.0 :`A` 1.0)))
      (`KismetArrayLibrary.Array_Add` (`self.reaction info list`) (make `/Game/DataTypes/Reaction_Info_Data_Structure` "CRYO" "GEO" "CRYSTALLIZE" 50 (struct :`R` 100.0 :`G` 100.0 :`A` 1.0))))
    (:`then_4`
      ;[1 1 1] pyro based reactions
      (`KismetArrayLibrary.Array_Add` (`self.reaction info list`) (make `/Game/DataTypes/Reaction_Info_Data_Structure` "PYRO" "CRYO" "MELT" 35 (struct :`R` 100.0 :`G` 10.000002 :`B` 10.000002 :`A` 1.0)))
      (`KismetArrayLibrary.Array_Add` (`self.reaction info list`) (make `/Game/DataTypes/Reaction_Info_Data_Structure` "PYRO" "ELECTRO" "OVERLOAD" 65 (struct :`R` 100.0 :`G` 10.000002 :`B` 99.999962 :`A` 1.0)))
      (`KismetArrayLibrary.Array_Add` (`self.reaction info list`) (make `/Game/DataTypes/Reaction_Info_Data_Structure` "PYRO" "ANEMO" "SWIRL" 25 (struct :`R` 10.000002 :`G` 99.999977 :`B` 100.0 :`A` 1.0)))
      (`KismetArrayLibrary.Array_Add` (`self.reaction info list`) (make `/Game/DataTypes/Reaction_Info_Data_Structure` "PYRO" "HYDRO" "VAPORIZE" 75 (struct :`B` 100.0 :`A` 1.0)))
      (`KismetArrayLibrary.Array_Add` (`self.reaction info list`) (make `/Game/DataTypes/Reaction_Info_Data_Structure` "PYRO" "GEO" "CRYSTALLIZE" 50 (struct :`R` 100.0 :`G` 100.0 :`A` 1.0)))
      (`KismetArrayLibrary.Array_Add` (`self.reaction info list`) (make `/Game/DataTypes/Reaction_Info_Data_Structure` "PYRO" "DENDRO" "BURNING" 35 (struct :`R` 100.0 :`G` 0.1 :`B` 0.1 :`A` 1.0))))))

(fn `prepare index to stage effect`
  (for (_array_element _array_index) (`/Game/Blueprints/Save_Data/Level_Effect_Save_Data_BP.level effects` (`self.level effect ref`))
    (if (and (`|EnumEquality` (`/Game/Blueprints/Gameplay_GM.Name Enum` (`self.As Gameplay GM`)) (break `/Game/DataTypes/GamePlay/Level_Effect_Data_Structure` _array_element)) (== (`/Game/Blueprints/Gameplay_GM.Stage` (`self.As Gameplay GM`)) (`.stage_14_3F4F13E14128DBF59768268FFFD82154` (break `/Game/DataTypes/GamePlay/Level_Effect_Data_Structure` _array_element))))
      (set `self.stage effect index` _array_index)
      (break))))

(fn `update damage percent based on stage effect`
  (params (name :type String) (percent :type Integer))
  (returns (`final percent` :type Integer))
  (for _array_element (break `/Game/DataTypes/GamePlay/Stage_Effect_Data_Structure` (`.effect_19_11140BA542612913F7980CA5873F2470` (break `/Game/DataTypes/GamePlay/Level_Effect_Data_Structure` (`|GetArrayItem` (`/Game/Blueprints/Save_Data/Level_Effect_Save_Data_BP.level effects` (`self.level effect ref`)) (`self.stage effect index`)))))
    (if (`KismetStringLibrary.EqualEqual_StrStr` (`local.name`) (break `/Game/DataTypes/GamePlay/Reaction_Effect_Data_Structure` _array_element))
      (return (+ (`local.percent`) (* (`local.percent`) (`.percentage_6_16C5D8324DFB72856E2361AAFE8962B2` (break `/Game/DataTypes/GamePlay/Reaction_Effect_Data_Structure` _array_element)) 0.01)))))
  (return (`local.percent`)))

(fn `update scoring and hp`
  (params (`in damage` :type Integer))
  (bind _as_enemy_base_bp (`self.As Enemy Base BP`))
  (bind _in_damage (`local.in damage`))
  (`|ExecutionSequence`
    (:`then_0`
      (if (> _in_damage 0)
        (`/Game/Blueprints/Main_GM.calculate total damage` (`self.As Gameplay GM`) _in_damage)))
    (:`then_1`
      (set `/Game/Blueprints/Obstacles/Enemy/Enemy_Base_BP.my current hp` (- (`/Game/Blueprints/Obstacles/Enemy/Enemy_Base_BP.my current hp` (`self.As Enemy Base BP`)) (`local.in damage`)) (`self.As Enemy Base BP`)))
    (:`then_2`
      (if (< (`/Game/Blueprints/Obstacles/Enemy/Enemy_Base_BP.my current hp` _as_enemy_base_bp) 0)
        (message `/Game/Blueprints/Interface/Kill_BPI.handle kill` _as_enemy_base_bp)))))