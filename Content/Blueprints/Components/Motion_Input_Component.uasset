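; Motion input component that turns the player's device tilt and gravity sensor readings into normalized forward and sideways axis values.
; GetMotion flags ButtonFacingFloor from the sign of gravity X and uses it to flip the clamped Tilt X for sideways.
; Forward comes from the absolute Tilt Y, via the GetOnlyValue helper, clamped and remapped to an inverted -1 to 1 range.
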(fn `get motion `
  (returns (forward :type "Float (double-precision)") (sideway :type "Float (double-precision)"))
  (locals (`temp forward` :type "Float (double-precision)") (`temp sideways` :type "Float (double-precision)") (`button facing floor` :type Boolean))
  (bind (_tilt _rotationrate _gravity) (`PlayerController.GetInputMotionState` (`GameplayStatics.GetPlayerController` 0)))
  (bind _returnvalue (* (.x _tilt) 100.0))
  (`|ExecutionSequence`
    (:`then_0`
      ;[1 1 1] gravity basis conditioning
      (set `local.button facing floor` (< (* (.x _gravity) 100.0) 0.0)))
    (:`then_1`
      ;[1 1 1] sideways
      (if (`local.button facing floor`)
        (set `local.temp sideways` (/ (`KismetMathLibrary.FClamp` _returnvalue -50.0 50.0) 50.0))
        (else
          (set `local.temp sideways` (/ (`KismetMathLibrary.FClamp` (* _returnvalue -1.0) -50.0 50.0) 50.0)))))
    (:`then_2`
      ;[1 1 1] Forward
      (set `local.temp forward` (* (- (/ (- (`KismetMathLibrary.FClamp` (* (`self.get only value` (.y _tilt)) 100.0) 50.0 100.0) 50.0) 25.0) 1.0) -1.0)))
    (:`then_3`
      (return (`local.temp forward`) (`local.temp sideways`)))))

(fn `get only value`
  (params (`in value` :type "Float (double-precision)"))
  (returns (magnitude :type "Float (double-precision)"))
  (if (> `in value` 0.0)
    (return `in value`)
    (else
      (return (* `in value` -1.0)))))