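; Obstacle viewer actor that displays an enemy or obstacle selected by key name and element name.
; HandleSpawning stores the selection, destroys attached Enemy_Base_BP actors, spawns the class mapped to the key, initializes it with the element and attaches it to the Arrow.
; A timeline started on BeginPlay animates the Arrow's relative Z, carrying the displayed actor.
; Tick respawns the stored selection whenever no enemy is attached.
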(event `self.ReceiveBeginPlay`
  (bind (_direction _z_track) (`Timeline|z timline` :!via `PlayFromStart`)
    (:`Update`
      (`SceneComponent.K2_SetRelativeLocation` (`self.Arrow`) (`KismetMathLibrary.MakeVector` 0.0 0.0 _z_track) false false))))

(event `self.ReceiveTick`
  (params (DeltaSeconds :type "Float (single-precision)"))
  (if (not (`self.is there any attached actor`))
    (`self.handle spawning` (`self.current keyname`) (`self.current element name`))))

(event `handle spawning`
  (params (`current keyname` :type String) (`current element name` :type String))
  (set `self.current keyname` `current keyname`)
  (set `self.current element name` `current element name`)
  (`|ExecutionSequence`
    (:`then_0`
      (for _array_element (`self.GetAttachedActors` true true)
        (bind _asenemy_base_bp (cast `/Game/Blueprints/Obstacles/Enemy/Enemy_Base_BP` _array_element))
        (`self.K2_DestroyActor` _asenemy_base_bp)))
    (:`then_1`
      (bind _returnvalue (`|SpawnActorFromClass` (`BlueprintMapLibrary.Map_Find` (`/Game/Blueprints/Library/Enemy_BFL.get keyname to classname`) (`self.current keyname`)) (`KismetMathLibrary.MakeTransform` (0.0 0.0 0.0)) "AlwaysSpawn" "MultiplyWithRoot" null (`self.current keyname`) false null))
      (`/Engine/EditorBlueprintResources/StandardMacros.IsValid` _returnvalue
        (:`Is Valid`
          (`/Game/Blueprints/Obstacles/Enemy/Enemy_Base_BP.init again` _returnvalue (`self.current element name`) false)
          (`self.K2_AttachToComponent` _returnvalue (`self.Arrow`) "None" "KeepRelative" "KeepRelative" "KeepRelative" true))))))

(fn `is there any attached actor`
  (returns (`return value` :type Boolean))
  (for _array_element (`self.GetAttachedActors` true true)
    (cast `/Game/Blueprints/Obstacles/Enemy/Enemy_Base_BP` _array_element)
    (return true))
  (return false))

(fn `UserConstructionScript`)