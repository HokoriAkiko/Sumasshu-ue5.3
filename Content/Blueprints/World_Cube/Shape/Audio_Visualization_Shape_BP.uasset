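; A shape Blueprint for audio visualization that stretches vertically with an amplitude value fed to it through an event.
; On BeginPlay it randomizes the root component's X and Y scale, stores that as the initial scale and picks a random response multiplier.
; The amplitude event sets only Z scale from the amplified input times that multiplier, so each instance reacts differently.
; A reset event restores the stored initial scale.
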(event `reset scale`
  (`SceneComponent.SetRelativeScale3D` (`self.DefaultSceneRoot`) (`self.initial scale`)))

(event `current amplitude`
  (params (`in q ` :type "Float (double-precision)"))
  (bind (_relativescale3d_x _relativescale3d_y) (`KismetMathLibrary.BreakVector` (`SceneComponent.RelativeScale3D` (`self.DefaultSceneRoot`))))
  (`SceneComponent.SetRelativeScale3D` (`self.DefaultSceneRoot`) (`KismetMathLibrary.MakeVector` _relativescale3d_x _relativescale3d_y (* (`self.scale`) (* `in q ` 20.0)))))

(event `self.ReceiveBeginPlay`
  (bind _returnvalue (`KismetMathLibrary.RandomFloatInRange` 0.25 1.0))
  (bind _defaultsceneroot (`self.DefaultSceneRoot`))
  (`SceneComponent.SetRelativeScale3D` _defaultsceneroot (`KismetMathLibrary.MakeVector` _returnvalue _returnvalue 1.0))
  (set `self.initial scale` (`SceneComponent.RelativeScale3D` _defaultsceneroot))
  (set `self.scale` (`KismetMathLibrary.RandomFloat`)))

(fn `UserConstructionScript`)