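; Limit_Parent_BP is a parent actor that builds a line of Limit_Child_BP boundary pieces and sets which wall they form.
; developelimit spawns children at fixed spacing along Y or X, depending on IsColumn, and attaches them to its root.
; The left, right and front wall events loop over attached actors and tell each child to take that wall position.
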(event `develope limit`
  (if (`self.is column`)
    (for _index (range 2 10)
      (bind _returnvalue (`|SpawnActorFromClass` "/Game/Blueprints/Limit/Limit_Child_BP.Limit_Child_BP_C" (`KismetMathLibrary.MakeTransform` (`KismetMathLibrary.MakeVector` 0.0 (`KismetMathLibrary.Conv_IntToDouble` (* _index 200)) -50.0)) "Undefined" "MultiplyWithRoot" null null))
      (`self.K2_AttachToComponent` _returnvalue (`self.DefaultSceneRoot`) "None" "KeepRelative" "KeepRelative" "KeepRelative" true))
    (else
      (for _index_2 (range 10)
        (bind _returnvalue_2 (`|SpawnActorFromClass` "/Game/Blueprints/Limit/Limit_Child_BP.Limit_Child_BP_C" (`KismetMathLibrary.MakeTransform` (`KismetMathLibrary.MakeVector` (`KismetMathLibrary.Conv_IntToDouble` (* _index_2 -200)) 0.0 -50.0)) "Undefined" "MultiplyWithRoot" null null))
        (`self.K2_AttachToComponent` _returnvalue_2 (`self.DefaultSceneRoot`) "None" "KeepRelative" "KeepRelative" "KeepRelative" true)))))

(event `parent is left wall`
  (for _array_element (`self.GetAttachedActors` true)
    (bind _aslimit_child_bp (cast `/Game/Blueprints/Limit/Limit_Child_BP` _array_element))
    (`/Game/Blueprints/Limit/Limit_Child_BP.left wall position` _aslimit_child_bp)))

(event `parent is right wall`
  (for _array_element (`self.GetAttachedActors` true)
    (bind _aslimit_child_bp (cast `/Game/Blueprints/Limit/Limit_Child_BP` _array_element))
    (`/Game/Blueprints/Limit/Limit_Child_BP.right wall position` _aslimit_child_bp)))

(event `parent is front wall`
  (for _array_element (`self.GetAttachedActors` true)
    (bind _aslimit_child_bp (cast `/Game/Blueprints/Limit/Limit_Child_BP` _array_element))
    (`/Game/Blueprints/Limit/Limit_Child_BP.front wall position` _aslimit_child_bp)))

(fn `UserConstructionScript`)