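; Simple_Cube_BP is a scrolling cube actor that gives its static mesh a random, tall-leaning scale at BeginPlay.
; Tick moves it along local negative X by a fixed, frame-rate-dependent step, without sweep.
; A countdown in Tick periodically calls DeleteIfTooFar, which destroys the actor past a negative world X limit or otherwise restarts the countdown.
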(event `self.ReceiveBeginPlay`
  (`SceneComponent.SetRelativeScale3D` (`self.StaticMesh`) (`KismetMathLibrary.MakeVector` (`KismetMathLibrary.RandomFloatInRange` 1.0 10.0) (`KismetMathLibrary.RandomFloatInRange` 1.0 10.0) (`KismetMathLibrary.RandomFloatInRange` 9.0 10.0))))

(event `self.ReceiveTick`
  (params (DeltaSeconds :type "Float (single-precision)"))
  (`|ExecutionSequence`
    (:`then_0`
      (bind _output_get (set `self.check time` (- (`self.check time`) DeltaSeconds)))
      (if (< _output_get 0.0)
        (`self.delete if too far`)))
    (:`then_1`
      (`self.K2_AddActorLocalOffset` (-10.0 0.0 0.0)))))

(event `delete if too far`
  (bind _returnvalue_x (`KismetMathLibrary.BreakVector` (`self.K2_GetActorLocation`)))
  (if (< _returnvalue_x -1000.0)
    (`self.K2_DestroyActor`)
    (else
      (set `self.check time` 1.0))))

(fn `UserConstructionScript`)