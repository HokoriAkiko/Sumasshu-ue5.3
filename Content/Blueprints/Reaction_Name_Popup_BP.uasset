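; Floating popup actor that displays a reaction name in a given color for a short time.
; On begin play it sets a two-second lifespan, passes the name and color to its Reaction_Name_Popup_Widget_BP, and calls that widget's parenting and animation handler.
; Every tick it moves upward by a fixed local offset, not scaled by delta time, so rise speed depends on frame rate.
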(event `self.ReceiveBeginPlay`
  (`|ExecutionSequence`
    (:`then_0`
      (`self.SetLifeSpan` 2.0))
    (:`then_1`
      (bind _asreaction_name_popup_widget_bp (cast `/Game/UI/Blueprints/Reaction_Name_Popup_Widget_BP` (`WidgetComponent.GetWidget` (`self.Widget`))))
      (set `/Game/UI/Blueprints/Reaction_Name_Popup_Widget_BP.reaction name` (`KismetTextLibrary.Conv_StringToText` (`self.reaction name`)) _asreaction_name_popup_widget_bp)
      (set `/Game/UI/Blueprints/Reaction_Name_Popup_Widget_BP.reaction color` (`self.reaction color`) _asreaction_name_popup_widget_bp)
      (`/Game/UI/Blueprints/Reaction_Name_Popup_Widget_BP.handle parenting and animation` _asreaction_name_popup_widget_bp self))))

(event `self.ReceiveTick`
  (params (DeltaSeconds :type "Float (single-precision)"))
  (`self.K2_AddActorLocalOffset` (0.0 0.0 10.0)))

(fn `UserConstructionScript`)