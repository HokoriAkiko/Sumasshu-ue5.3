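; Base Blueprint for enemy obstacles that carry an element and take damage from projectiles and blasts.
; On BeginPlay or InitAgain, it picks a random or named element from ElementAssignmentComponent's ColorMap unless disabled, then selects the matching Niagara icon material.
; Hit events delegate damage to DamageHandlerComponent, refresh HP percent and set GotHit, with a sound on projectile hits.
; HandleKill is an empty event marked to be kept.
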(event `/Game/Blueprints/Interface/Initialization_BPI.init again`
  (params (`selected element name` :type String))
  (`self.decide element` `selected element name`)
  (`self.set my element ns material`)
  (`self.calculate hp percent`))

(event `self.ReceiveBeginPlay`
  (`self.decide element` "")
  (`self.set my element ns material`)
  (`self.calculate hp percent`))

(event `/Game/Blueprints/Interface/Kill_BPI.handle kill`
  ;[1 1 1] do not delete
)

(event `/Game/Blueprints/Interface/Ball_Projectile_On_Hit_BPI.hit by projectile`
  (params (`damage configuration` :type "/Game/DataTypes/Projectile_Damage_Configuration_Data_Structure Structure") (`projectile element name` :type "String (by ref)"))
  (`|ExecutionSequence`
    (:`then_0`
      (`/Game/Blueprints/Components/Damage_Handler_Component.handle projectile damage` (`self.Damage_Handler_Component`) `damage configuration` `projectile element name` (`/Game/Blueprints/Components/Element_Assignment_Component.selected element name` (`self.Element_Assignment_Component`))))
    (:`then_1`
      (`self.calculate hp percent`))
    (:`then_2`
      (if (not (`self.got hit`))
        (set `self.got hit` true)))
    (:`then_3`
      (`GameplayStatics.PlaySound2D` "/Game/Audio/cue/enemy_on_hit_Cue.enemy_on_hit_Cue" 1.0 1.0 0.0 null null))))

(event `/Game/Blueprints/Interface/Blast_BPI.hit by blast`
  (params (`blast configuration` :type "/Game/DataTypes/Blast_Damage_Configuration_Data_Structure Structure"))
  (`|ExecutionSequence`
    (:`then_0`
      (`/Game/Blueprints/Components/Damage_Handler_Component.handle blast damage` (`self.Damage_Handler_Component`) `blast configuration`))
    (:`then_1`
      (`self.calculate hp percent`))
    (:`then_2`
      (if (not (`self.got hit`))
        (set `self.got hit` true)))))

(fn `calculate hp percent`
  (set `self.my hp percent` (/ (* (`self.my current hp`) 100) (`self.my max hp`))))

(fn `decide element`
  (params (`selected element name` :type String))
  (locals (`temp index` :type Integer :default 0))
  (bind _selected_element_name (`local.selected element name`))
  (bind _color_map (`/Game/Blueprints/Components/Element_Assignment_Component.color map` (`self.Element_Assignment_Component`)))
  (bind _color_map_2 (`/Game/Blueprints/Components/Element_Assignment_Component.color map` (`self.Element_Assignment_Component`)))
  (if (not (`/Game/Blueprints/Components/Element_Assignment_Component.disabled` (`self.Element_Assignment_Component`)))
    (`|ExecutionSequence`
      (:`then_0`
        (if (== (`KismetStringLibrary.Len` _selected_element_name) 0)
          (set `local.temp index` (`KismetMathLibrary.RandomIntegerInRange` 0 (- (`BlueprintMapLibrary.Map_Length` _color_map_2) 1)))
          (else
            (bind _keys (`BlueprintMapLibrary.Map_Keys` _color_map_2))
            (set `local.temp index` (`KismetArrayLibrary.Array_Find` _keys _selected_element_name)))))
      (:`then_1`
        (bind _keys_2 (`BlueprintMapLibrary.Map_Keys` _color_map))
        (bind _output (`|GetArrayItem` _keys_2 (`local.temp index`)))
        (set `/Game/Blueprints/Components/Element_Assignment_Component.selected element name` _output (`self.Element_Assignment_Component`))
        (set `/Game/Blueprints/Components/Element_Assignment_Component.selected element color` (`BlueprintMapLibrary.Map_Find` _color_map _output) (`self.Element_Assignment_Component`))))))

(fn `set my element ns material`
  (switch `string` (`/Game/Blueprints/Components/Element_Assignment_Component.selected element name` (`self.Element_Assignment_Component`))
    (:`PYRO`
      (set `self.element ns material` "/Game/My_Textures/logo/NS/Pyro_Icon_NS_Material.Pyro_Icon_NS_Material"))
    (:`ELECTRO`
      (set `self.element ns material` "/Game/My_Textures/logo/NS/Electro_Icon_NS_Material.Electro_Icon_NS_Material"))
    (:`HYDRO`
      (set `self.element ns material` "/Game/My_Textures/logo/NS/Hydro_Icon_NS_Material.Hydro_Icon_NS_Material"))
    (:`CRYO`
      (set `self.element ns material` "/Game/My_Textures/logo/NS/Cryo_Icon_NS_Material.Cryo_Icon_NS_Material"))
    (:`GEO`
      (set `self.element ns material` "/Game/My_Textures/logo/NS/Geo_Icon_NS_Material.Geo_Icon_NS_Material"))
    (:`ANEMO`
      (set `self.element ns material` "/Game/My_Textures/logo/NS/Anemo_Icon_NS_Material.Anemo_Icon_NS_Material"))
    (:`DENDRO`
      (set `self.element ns material` "/Game/My_Textures/logo/NS/Dendro_Icon_NS_Material.Dendro_Icon_NS_Material"))))

(fn `UserConstructionScript`)