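; Ball projectile for the maze paddle game that bounces around, damages what it hits and takes on the paddle's element.
; Hits send damage and element through an interface, adjust velocity via an impulse component (Enemy_4 absorbs impulse), recopy element, color and VFX from the paddle, and check for all enemies dead.
; Leaving bounds or being blasted notifies the paddle, re-enables the launch button disabled at spawn, decrements projectile count in certain modes and destroys the ball.
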(event `init refs`
  (`|ExecutionSequence`
    (:`then_0`
      (bind _outactors (`GameplayStatics.GetAllActorsOfClass` "/Game/Blueprints/Maze/Maze_BP.Maze_BP_C"))
      (set `self.my maze` (`|GetArrayItem` _outactors)))
    (:`then_1`
      (bind _foundwidgets (`WidgetBlueprintLibrary.GetAllWidgetsOfClass` "/Game/UI/Blueprints/Gameplay/Gameplay_Main_Widget_BP.Gameplay_Main_Widget_BP_C" false))
      (for _array_element _foundwidgets
        (`/Game/UI/Blueprints/Gameplay/Launch_Ball_Widget_BP.disable launch button` (`/Game/UI/Blueprints/Gameplay/Gameplay_Main_Widget_BP.Launch_Ball_Widget_BP` _array_element))))
    (:`then_2`
      (bind _asgameplay_gm (cast `/Game/Blueprints/Gameplay_GM` (`GameplayStatics.GetGameMode`)))
      (set `self.As Gameplay GM` _asgameplay_gm))))

(event `self.ReceiveBeginPlay`
  (`parent.ReceiveBeginPlay`)
  (`self.init refs`)
  (bind _aspaddle_bp (cast `/Game/Blueprints/Maze/Paddle_BP` (`ChildActorComponent.ChildActor` (`/Game/Blueprints/Maze/Maze_BP.Paddle` (`self.my maze`)))))
  (`self.Copy Element from Other Actor` _aspaddle_bp)
  (`self.update ball color`)
  (`self.update vfx as per state`))

(event `self.ReceiveTick`
  (params (DeltaSeconds :type "Float (single-precision)"))
  (`parent.ReceiveTick` DeltaSeconds)
  (`self.kill check` false))

(event `self.collider.OnComponentHit`
  (params (HitComponent :type "PrimitiveComponent Object Reference") (OtherActor :type "Actor Object Reference") (OtherComp :type "PrimitiveComponent Object Reference") (NormalImpulse :type "Vector Structure") (Hit :type "HitResult Structure (by ref)"))
  (`self.handle hit` OtherActor))

(event `/Game/Blueprints/Interface/Blast_BPI.hit by blast`
  (params (`blast configuration` :type "/Game/DataTypes/Blast_Damage_Configuration_Data_Structure Structure"))
  (`self.kill check` true))

(fn `handle hit`
  (params (`other actor` :type "Actor Object Reference"))
  (bind _projectile_impulse_component_bp (`self.Projectile_Impulse_Component_BP`))
  (`|ExecutionSequence`
    (:`then_0`
      (`GameplayStatics.SpawnSoundAtLocation` "/Game/Interface_And_Item_Sounds/WAV/Coins_01_Cue.Coins_01_Cue" (`self.K2_GetActorLocation`) (struct) 1.0 1.0 0.0 null null)
      (`|SpawnActorFromClass` "/Game/Blueprints/VFX/Ball_On_Hit_VFX_P.Ball_On_Hit_VFX_P_C" (`KismetMathLibrary.MakeTransform` (`SceneComponent.K2_GetComponentLocation` (`self.collider`))) "Undefined" "MultiplyWithRoot" null null))
    (:`then_1`
      (bind _other_actor (`local.other actor`)
        (:`then`
          (if (`KismetSystemLibrary.DoesImplementInterface` _other_actor "/Game/Blueprints/Interface/Ball_Projectile_On_Hit_BPI.Ball_Projectile_On_Hit_BPI_C")
            (message `/Game/Blueprints/Interface/Ball_Projectile_On_Hit_BPI.hit by projectile` _other_actor (`self.damage configuration`) (`/Game/Blueprints/Components/Element_Assignment_Component.selected element name` (`self.Element_Assignment_Component`)))))
        (:`else`)))
    (:`then_2`
      (bind _other_actor_2 (`local.other actor`)
        (:`then`
          (cast `/Game/Blueprints/Obstacles/Enemy/Enemy_4_BP` _other_actor_2
            (:`then`
              (`/Game/Blueprints/Components/Projectile_Impulse_Component_BP.impulse absorbed` _projectile_impulse_component_bp))
            (:`CastFailed`
              _))
          (`/Game/Blueprints/Components/Projectile_Impulse_Component_BP.handle velocity` _projectile_impulse_component_bp))
        (:`else`)))
    (:`then_3`
      (bind _other_actor_3 (`local.other actor`)
        (:`then`
          (bind _aspaddle_bp (cast `/Game/Blueprints/Maze/Paddle_BP` _other_actor_3))
          (`self.Copy Element from Other Actor` _aspaddle_bp)
          (`self.update ball color`)
          (`self.update vfx as per state`))
        (:`else`)))
    (:`then_4`
      (`/Game/Blueprints/Components/Gameplay_Helper_Component_BP.on all enemies death` (`/Game/Blueprints/Gameplay_GM.Gameplay_Helper_Component_BP` (`self.As Gameplay GM`))))))

(fn `kill check`
  (params (`got hit by blast` :type Boolean))
  (bind (_returnvalue_x _returnvalue_y) (`KismetMathLibrary.BreakVector` (`SceneComponent.K2_GetComponentLocation` (`self.collider`))))
  (if (or (< _returnvalue_x -2500.0) (> _returnvalue_x 500.0) (< _returnvalue_y -500.0) (`local.got hit by blast`))
    (`|ExecutionSequence`
      (:`then_0`
        (bind _aspaddle_bp (cast `/Game/Blueprints/Maze/Paddle_BP` (`ChildActorComponent.ChildActor` (`/Game/Blueprints/Maze/Maze_BP.Paddle` (`self.my maze`)))))
        (`/Game/Blueprints/Maze/Paddle_BP.on projectile death` _aspaddle_bp))
      (:`then_1`
        (bind _foundwidgets (`WidgetBlueprintLibrary.GetAllWidgetsOfClass` "/Game/UI/Blueprints/Gameplay/Gameplay_Main_Widget_BP.Gameplay_Main_Widget_BP_C" false))
        (for _array_element _foundwidgets
          (`/Game/UI/Blueprints/Gameplay/Launch_Ball_Widget_BP.enable launch button` (`/Game/UI/Blueprints/Gameplay/Gameplay_Main_Widget_BP.Launch_Ball_Widget_BP` _array_element))))
      (:`then_2`
        (`self.update projectile count`))
      (:`then_3`
        (`self.K2_DestroyActor`)
        (`GameplayStatics.PlaySound2D` "/Game/Interface_And_Item_Sounds/WAV/Pop_07_Cue.Pop_07_Cue" 1.0 1.0 0.0 null null)))))

(fn `update projectile count`
  (bind _as_gameplay_gm (`self.As Gameplay GM`))
  (switch `/Game/DataTypes/UI/Game_Mode_Name_ENUM` (`/Game/Blueprints/Gameplay_GM.Name Enum` _as_gameplay_gm)
    (:`NewEnumerator1`
      _)
    (:`NewEnumerator2`
      _))
  (`/Engine/EditorBlueprintResources/StandardMacros.DecrementInt` (`/Game/Blueprints/Components/Gameplay_Helper_Component_BP.projectile count` (`/Game/Blueprints/Gameplay_GM.Gameplay_Helper_Component_BP` _as_gameplay_gm))))

(fn `UserConstructionScript`
  (`parent.UserConstructionScript`))