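; Actor component that provides lookup data for seven elements (Pyro, Hydro, Cryo, Electro, Anemo, Geo, Dendro).
; On BeginPlay it builds an element name list plus name-keyed maps for colors, UI icon materials and raw icons.
; The color map draws its values from MakeColorList.
; When Disabled is set, it skips the tables and only sets the selected element color to a fixed light grey.
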(event `self.ReceiveBeginPlay`
  (if (`self.disabled`)
    (set `self.selected element color` (make `Color` 200 200 200 1))
    (else
      (`|ExecutionSequence`
        (:`then_0`
          (`self.make element name list`))
        (:`then_1`
          (`self.make color map`))
        (:`then_2`
          (`self.make ui icon map`))
        (:`then_3`
          (`self.make raw icon map`))))))

(fn `make color map`
  (locals (`temp color list` :type "/Game/DataTypes/Color_List Structure"))
  (`BlueprintMapLibrary.Map_Clear` (`self.color map`))
  (bind _output_get (set `local.temp color list` (make `/Game/DataTypes/Color_List` (struct :`A` 1))))
  (bind (_immune _hydro _dendro _anemo _pyro _electro _geo _cryo) (break `/Game/DataTypes/Color_List` _output_get))
  (`BlueprintMapLibrary.Map_Add` (`self.color map`) "HYDRO" _hydro)
  (`BlueprintMapLibrary.Map_Add` (`self.color map`) "DENDRO" _dendro)
  (`BlueprintMapLibrary.Map_Add` (`self.color map`) "ANEMO" _anemo)
  (`BlueprintMapLibrary.Map_Add` (`self.color map`) "PYRO" _pyro)
  (`BlueprintMapLibrary.Map_Add` (`self.color map`) "ELECTRO" _electro)
  (`BlueprintMapLibrary.Map_Add` (`self.color map`) "GEO" _geo)
  (`BlueprintMapLibrary.Map_Add` (`self.color map`) "CRYO" _cryo))

(fn `make element name list`
  (`KismetArrayLibrary.Array_Clear` (`self.element name list`))
  (`KismetArrayLibrary.Array_Add` (`self.element name list`) "PYRO")
  (`KismetArrayLibrary.Array_Add` (`self.element name list`) "HYDRO")
  (`KismetArrayLibrary.Array_Add` (`self.element name list`) "CRYO")
  (`KismetArrayLibrary.Array_Add` (`self.element name list`) "ELECTRO")
  (`KismetArrayLibrary.Array_Add` (`self.element name list`) "ANEMO")
  (`KismetArrayLibrary.Array_Add` (`self.element name list`) "GEO")
  (`KismetArrayLibrary.Array_Add` (`self.element name list`) "DENDRO"))

(fn `make raw icon map`
  (`BlueprintMapLibrary.Map_Clear` (`self.raw icon map`))
  (`BlueprintMapLibrary.Map_Add` (`self.raw icon map`) "ANEMO" "/Game/My_Textures/logo/anemo_icon.anemo_icon")
  (`BlueprintMapLibrary.Map_Add` (`self.raw icon map`) "PYRO" "/Game/My_Textures/logo/pyro_icon.pyro_icon")
  (`BlueprintMapLibrary.Map_Add` (`self.raw icon map`) "HYDRO" "/Game/My_Textures/logo/hydro_icon.hydro_icon")
  (`BlueprintMapLibrary.Map_Add` (`self.raw icon map`) "CRYO" "/Game/My_Textures/logo/cryo_icon.cryo_icon")
  (`BlueprintMapLibrary.Map_Add` (`self.raw icon map`) "GEO" "/Game/My_Textures/logo/geo_icon.geo_icon")
  (`BlueprintMapLibrary.Map_Add` (`self.raw icon map`) "DENDRO" "/Game/My_Textures/logo/dendro_icon.dendro_icon")
  (`BlueprintMapLibrary.Map_Add` (`self.raw icon map`) "ELECTRO" "/Game/My_Textures/logo/electro_icon.electro_icon"))

(fn `make ui icon map`
  (`BlueprintMapLibrary.Map_Clear` (`self.ui icon map`))
  (`BlueprintMapLibrary.Map_Add` (`self.ui icon map`) "PYRO" "/Game/My_Textures/logo/Pyro_Icon_UI_Material.Pyro_Icon_UI_Material")
  (`BlueprintMapLibrary.Map_Add` (`self.ui icon map`) "HYDRO" "/Game/My_Textures/logo/Hydro_Icon_UI_Material.Hydro_Icon_UI_Material")
  (`BlueprintMapLibrary.Map_Add` (`self.ui icon map`) "CRYO" "/Game/My_Textures/logo/Cryo_Icon_UI_Material.Cryo_Icon_UI_Material")
  (`BlueprintMapLibrary.Map_Add` (`self.ui icon map`) "ELECTRO" "/Game/My_Textures/logo/Electro_Icon_UI_Material.Electro_Icon_UI_Material")
  (`BlueprintMapLibrary.Map_Add` (`self.ui icon map`) "ANEMO" "/Game/My_Textures/logo/Anemo_Icon_UI_Material.Anemo_Icon_UI_Material")
  (`BlueprintMapLibrary.Map_Add` (`self.ui icon map`) "GEO" "/Game/My_Textures/logo/Geo_Icon_UI_Material.Geo_Icon_UI_Material")
  (`BlueprintMapLibrary.Map_Add` (`self.ui icon map`) "DENDRO" "/Game/My_Textures/logo/Dendro_Icon_UI_Material.Dendro_Icon_UI_Material"))