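; Spawner actor that scatters Home_Level_Background_Shape_BP actors, apparently as background for the home level.
; On BeginPlay it walks a 50 by 50 index grid and spawns a shape in roughly 70% of the cells.
; Each index is multiplied by a random distance, so shapes extend along positive X and fan out to both sides in Y, at the spawner's height.
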(event `self.ReceiveBeginPlay`
  (for _index (range 1 51)
    (for _index_2 (range 1 51)
      (if (> (`KismetMathLibrary.RandomFloat`) 0.3)
        (`|SpawnActorFromClass` "/Game/Blueprints/World_Cube/Shape/Home_Level_Background_Shape_BP.Home_Level_Background_Shape_BP_C" (`KismetMathLibrary.MakeTransform` (+ (`self.K2_GetActorLocation`) (`KismetMathLibrary.MakeVector` (* _index (`KismetMathLibrary.RandomFloatInRange` 500.0 2000.0)) (* _index_2 (`KismetMathLibrary.RandomFloatInRange` -1000.0 1000.0))))) "Undefined" "OverrideRootScale" null null)))))

(fn `UserConstructionScript`)