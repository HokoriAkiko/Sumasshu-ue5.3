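; Actor component that shakes its owner's box component as a hit reaction on enemies.
; BeginPlay caches the owner as Actor_Main_BP and Enemy_Base_BP.
; While GotHit and ReactionOccurred are set and shaking is not disabled, Tick randomizes the box's relative location on axes flagged by DirectionVector, holding the others at OriginalLocation.
; Once ShakeDuration elapses, it clears GotHit, restores OriginalLocation and resets the timer.
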(event `self.ReceiveBeginPlay`
  (bind _returnvalue (`self.GetOwner`))
  (`|ExecutionSequence`
    (:`then_0`
      (bind _asactor_main_bp (cast `/Game/Blueprints/Actor_Main_BP` _returnvalue))
      (set `self.As Actor Main BP` _asactor_main_bp))
    (:`then_1`
      (bind _asenemy_base_bp (cast `/Game/Blueprints/Obstacles/Enemy/Enemy_Base_BP` _returnvalue))
      (set `self.As Enemy Base BP` _asenemy_base_bp))))

(event `self.ReceiveTick`
  (params (DeltaSeconds :type "Float (single-precision)"))
  (if (and (`/Game/Blueprints/Actor_Main_BP.got hit` (`self.As Actor Main BP`)) (`/Game/Blueprints/Obstacles/Enemy/Enemy_Base_BP.reaction occured` (`self.As Enemy Base BP`)) (not (`self.disabled`)))
    (bind _output_get (set `self.shake counter` (+ DeltaSeconds (`self.shake counter`))))
    (if (> _output_get (`self.shake duration`))
      (set `/Game/Blueprints/Actor_Main_BP.got hit` false (`self.As Actor Main BP`))
      (`self.after shake`)
      (set `self.shake counter` 0.0)
      (else
        (`self.shake me`)))))

(fn `after shake`
  (`SceneComponent.K2_SetRelativeLocation` (`Actor.GetComponentByClass` (`self.GetOwner`) "/Script/Engine.BoxComponent") (`self.original location`) false false))

(fn `shake me`
  (locals (temp :type "Vector Structure"))
  (bind (_temp_x _temp_y) (`KismetMathLibrary.BreakVector` (`local.temp`)))
  (bind _original_location_x (`KismetMathLibrary.BreakVector` (`self.original location`)))
  (bind _temp_x_2 (`KismetMathLibrary.BreakVector` (`local.temp`)))
  (bind (_original_location_x_2 _original_location_y) (`KismetMathLibrary.BreakVector` (`self.original location`)))
  (bind (_direction_vector_x _direction_vector_y _direction_vector_z) (`KismetMathLibrary.BreakVector` (`self.direction vector`)))
  (bind (_original_location_x_3 _original_location_y_2 _original_location_z) (`KismetMathLibrary.BreakVector` (`self.original location`)))
  (`|ExecutionSequence`
    (:`then_0`
      (if (== _direction_vector_x 1.0)
        (set `local.temp` (`KismetMathLibrary.MakeVector` (`KismetMathLibrary.RandomFloatInRange` (`self.range min`) (`self.range max`))))
        (else
          (set `local.temp` (`KismetMathLibrary.MakeVector` _original_location_x)))))
    (:`then_1`
      (if (== _direction_vector_y 1.0)
        (set `local.temp` (`KismetMathLibrary.MakeVector` _temp_x_2 (`KismetMathLibrary.RandomFloatInRange` (`self.range min`) (`self.range max`))))
        (else
          (set `local.temp` (`KismetMathLibrary.MakeVector` _temp_x_2 _original_location_y)))))
    (:`then_2`
      (if (== _direction_vector_z 1.0)
        (set `local.temp` (`KismetMathLibrary.MakeVector` _temp_x _temp_y (`KismetMathLibrary.RandomFloatInRange` (`self.range min`) (`self.range max`))))
        (else
          (set `local.temp` (`KismetMathLibrary.MakeVector` _temp_x _temp_y _original_location_z)))))
    (:`then_3`
      (`SceneComponent.K2_SetRelativeLocation` (`Actor.GetComponentByClass` (`self.GetOwner`) "/Script/Engine.BoxComponent") (`local.temp`) false false))))