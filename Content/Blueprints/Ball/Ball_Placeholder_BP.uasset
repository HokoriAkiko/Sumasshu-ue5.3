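; Placeholder ball Blueprint that mirrors the elemental state of the paddle.
; On BeginPlay it runs the parent logic, finds the first Paddle_BP in the level and copies its element.
; It then updates the ball color and state-based VFX.
; The switchelement event re-runs the same lookup and refresh sequence, while Tick is disabled.
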(event `self.ReceiveBeginPlay`
  (`parent.ReceiveBeginPlay`)
  (bind _outactors (`GameplayStatics.GetAllActorsOfClass` "/Game/Blueprints/Maze/Paddle_BP.Paddle_BP_C" :!label _label))
  (`self.Copy Element from Other Actor` (`|GetArrayItem` _outactors))
  (`self.update ball color`)
  (`self.update vfx as per state`))

(event `switch element`
  (goto _label))

(fn `UserConstructionScript`
  (`parent.UserConstructionScript`))