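; Blueprint function library that serves as a static data catalogue for the game's five enemy types, keyed E1 to E5.
; Separate getters return maps from key to UI icon data, display name, lore text, enemy Blueprint class, and defeat hint.
; Each getter clears and rebuilds its map in code on every call, so the enemy definitions are hardcoded here rather than in a data table.
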(fn `get keyname icon map`
  (returns (`return keyname icon map` :type "Map of String to /Game/DataTypes/GamePlay/Enemy_Info_Dup_Data_Structure Structure"))
  (locals (`keyname icon map` :type "Map of String to /Game/DataTypes/GamePlay/Enemy_Info_Dup_Data_Structure Structure"))
  (`|ExecutionSequence`
    (:`then_0`
      (`BlueprintMapLibrary.Map_Clear` (`local.keyname icon map`))
      (`BlueprintMapLibrary.Map_Add` (`local.keyname icon map`) "E1" (make `/Game/DataTypes/GamePlay/Enemy_Info_Dup_Data_Structure` "E1" "/Game/My_Textures/shapes/Enemy_Type_1_UI_Material.Enemy_Type_1_UI_Material" "E1 Context..." "E1"))
      (`BlueprintMapLibrary.Map_Add` (`local.keyname icon map`) "E2" (make `/Game/DataTypes/GamePlay/Enemy_Info_Dup_Data_Structure` "E2" "/Game/My_Textures/shapes/Enemy_Type_2_UI_Material.Enemy_Type_2_UI_Material" "E2 Context..." "E2"))
      (`BlueprintMapLibrary.Map_Add` (`local.keyname icon map`) "E3" (make `/Game/DataTypes/GamePlay/Enemy_Info_Dup_Data_Structure` "E3" "/Game/My_Textures/shapes/Enemy_Type_3_UI_Material.Enemy_Type_3_UI_Material" "E3 Context..." "E3"))
      (`BlueprintMapLibrary.Map_Add` (`local.keyname icon map`) "E4" (make `/Game/DataTypes/GamePlay/Enemy_Info_Dup_Data_Structure` "E4" "/Game/My_Textures/shapes/Enemy_Type_4_UI_Material.Enemy_Type_4_UI_Material" "E4 Context..." "E4"))
      (`BlueprintMapLibrary.Map_Add` (`local.keyname icon map`) "E5" (make `/Game/DataTypes/GamePlay/Enemy_Info_Dup_Data_Structure` "E5" "/Game/My_Textures/shapes/Enemy_Type_5_UI_Material.Enemy_Type_5_UI_Material" "E5 Context..." "E5")))
    (:`then_1`
      (return (`local.keyname icon map`)))))

(fn `get keyname to classname`
  (returns (`keyname to class name map` :type "Map of String to /Game/Blueprints/Obstacles/Enemy/Enemy_Base_BP Class Reference"))
  (locals (map :type "Map of String to /Game/Blueprints/Obstacles/Enemy/Enemy_Base_BP Class Reference"))
  (`|ExecutionSequence`
    (:`then_0`
      (`BlueprintMapLibrary.Map_Clear` (`local.map`))
      (`BlueprintMapLibrary.Map_Add` (`local.map`) "E1" "/Game/Blueprints/Obstacles/Enemy/Enemy_1_BP.Enemy_1_BP_C")
      (`BlueprintMapLibrary.Map_Add` (`local.map`) "E2" "/Game/Blueprints/Obstacles/Enemy/Enemy_2_BP.Enemy_2_BP_C")
      (`BlueprintMapLibrary.Map_Add` (`local.map`) "E3" "/Game/Blueprints/Obstacles/Enemy/Enemy_3_BP.Enemy_3_BP_C")
      (`BlueprintMapLibrary.Map_Add` (`local.map`) "E4" "/Game/Blueprints/Obstacles/Enemy/Enemy_4_BP.Enemy_4_BP_C")
      (`BlueprintMapLibrary.Map_Add` (`local.map`) "E5" "/Game/Blueprints/Obstacles/Enemy/Enemy_5_BP.Enemy_5_BP_C"))
    (:`then_1`
      (return (`local.map`)))))

(fn `get keyname to context`
  (returns (`keyname to context` :type "Map of String to String"))
  (locals (`temp map` :type "Map of String to String"))
  (`|ExecutionSequence`
    (:`then_0`
      (`BlueprintMapLibrary.Map_Clear` (`local.temp map`))
      (`BlueprintMapLibrary.Map_Add` (`local.temp map`) "E1" "A fundamental obstacle of unknown origin. Each pulsates with the essence of its element, awaiting the kinetic force of the “Quantum Spheroid” to shatter its crystalline structure. As the shard fractures, it releases a burst of elemental energy.")
      (`BlueprintMapLibrary.Map_Add` (`local.temp map`) "E2" "A formidable obstacle fortified within a cubical framework, each face pulsating with the essence an elemental affinities. Guarded by arcane barriers and imbued with elemental resilience, requiring strategic manipulation of elemental strengths and weaknesses. Before the final strike can be dealt to its core, the player must first breach its formidable defenses by exploiting elemental vulnerabilities and deploying tactical prowess.")
      (`BlueprintMapLibrary.Map_Add` (`local.temp map`) "E3" "Deep within the labyrinth of forgotten ruins, a cubic mesh hums with ancient energy, its surface etched with cryptic patterns that flicker in the shadows. Once a relic of a lost civilization, it now stands as a silent guardian, impervious to the ravages of time. However, when struck by a projectile, its dormant defenses awaken. The impact reverberates through its crystalline structure, channeling the force into shimmering fractures. The physical damage penetrates the barrier, but the mesh seems to absorb the energy, as though it is feeding on the very power that seeks to destroy it.")
      (`BlueprintMapLibrary.Map_Add` (`local.temp map`) "E4" "A relentless foe poised to disrupt the flow of kinetic energy. Infused with elemental energy, Demolisher absorbs the momentum of any Quantum Spheroid that dares to challenge its domain.")
      (`BlueprintMapLibrary.Map_Add` (`local.temp map`) "E5" "A cunning adversary concealed within an enigmatic cube, infused with elemental energy. Upon its demise, obliterates not only itself but also Quantum Spheroid caught within its explosive radius."))
    (:`then_1`
      (return (`local.temp map`)))))

(fn `get keyname to defeat hint map`
  (returns (`hint map` :type "Map of String to String"))
  (locals (map :type "Map of String to String"))
  (`|ExecutionSequence`
    (:`then_0`
      (`BlueprintMapLibrary.Map_Clear` (`local.map`))
      (`BlueprintMapLibrary.Map_Add` (`local.map`) "E1" "Vulnerable to elemental reactions")
      (`BlueprintMapLibrary.Map_Add` (`local.map`) "E2" "Defense is decreased once the guard is down. Vulnerable to elemental reactions")
      (`BlueprintMapLibrary.Map_Add` (`local.map`) "E3" "Vulnerable to physical impacts")
      (`BlueprintMapLibrary.Map_Add` (`local.map`) "E4" "Absorbs energy of quantum spheroid on impact. Vulnerable to elemental reactions")
      (`BlueprintMapLibrary.Map_Add` (`local.map`) "E5" "Explodes on destrucion dealing damage to everyone around. Vulnerale to elemental reacrtions"))
    (:`then_1`
      (return (`local.map`)))))

(fn `get keyname to in game name`
  (returns (`return keyname to in game name map` :type "Map of String to String"))
  (locals (`temp map` :type "Map of String to String"))
  (`|ExecutionSequence`
    (:`then_0`
      (`BlueprintMapLibrary.Map_Clear` (`local.temp map`))
      (`BlueprintMapLibrary.Map_Add` (`local.temp map`) "E1" "Cubic Shatter")
      (`BlueprintMapLibrary.Map_Add` (`local.temp map`) "E2" "Armoured")
      (`BlueprintMapLibrary.Map_Add` (`local.temp map`) "E3" "Kinect")
      (`BlueprintMapLibrary.Map_Add` (`local.temp map`) "E4" "Demolisher")
      (`BlueprintMapLibrary.Map_Add` (`local.temp map`) "E5" "Spheric Blast"))
    (:`then_1`
      (return (`local.temp map`)))))