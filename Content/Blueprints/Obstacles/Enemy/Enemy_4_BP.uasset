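; Elemental enemy obstacle, extending a parent enemy, that steals the impulse of any projectile hit regardless of reaction.
; Its Body material takes the assigned element's color on BeginPlay and re-initialization.
; Projectile hits trigger a timeline animating the material's wind intensity, and a kill flag lets the timeline's finish destroy the actor.
; Projectile and blast hits spawn status popups at the collider: "Stealing Impulse" or "Explosive Impact".
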(event `handle timeline`
  (if (not (`self.is hit animation playing`))
    (if (`self.event on kill`)
      (bind (_direction _wind_intensity_track) (`Timeline|on hit timeline` :!via `Stop` :!label _label)
        (:`Update`
          (`self.on hit material ` _wind_intensity_track))
        (:`Finished`
          (set `self.is hit animation playing` false)
          (if (`self.event on kill`)
            (`self.K2_DestroyActor`))))
      (else
        (set `self.is hit animation playing` true)
        (goto _label :!via `PlayFromStart`)))))

(event `/Game/Blueprints/Interface/Initialization_BPI.init again`
  (params (`selected element name` :type String) (`in memory` :type Boolean))
  (`parent.init again` `selected element name` false)
  (`self.set material as per element color` :!label _label_2))

(event `self.ReceiveBeginPlay`
  (`parent.ReceiveBeginPlay`)
  (goto _label_2))

(event `/Game/Blueprints/Interface/Kill_BPI.handle kill`
  (`parent.handle kill`)
  (set `self.event on kill` true))

(event `/Game/Blueprints/Interface/Blast_BPI.hit by blast`
  (params (`blast configuration` :type "/Game/DataTypes/Blast_Damage_Configuration_Data_Structure Structure"))
  (`parent.hit by blast` `blast configuration`)
  (`self.handle spawning of vfx` "Explosive Impact"))

(event `/Game/Blueprints/Interface/Ball_Projectile_On_Hit_BPI.hit by projectile`
  (params (`damage configuration` :type "/Game/DataTypes/Projectile_Damage_Configuration_Data_Structure Structure") (`projectile element name` :type "String (by ref)"))
  (`parent.hit by projectile` `damage configuration` `projectile element name`)
  (`|ExecutionSequence`
    (:`then_0`
      ;[1 1 1] this type of enemy doesnt care if reaction occured or not , just steal the impluse
      (`self.handle timeline`))
    (:`then_1`
      (`self.handle spawning of vfx` "Stealing Impulse"))))

(fn `handle spawning of vfx`
  (params (status :type Text :default "NSLOCTEXT(\"[BC0CF52A956C5008F69F91BDE16E201C]\", \"3C96B5FA41802A4A6B5D1C9C59CF3EE8\", \"Default Status\")"))
  (`|ExecutionSequence`
    (:`then_0`
      (if (!= (`KismetStringLibrary.Len` (`KismetTextLibrary.Conv_TextToString` (`local.status`))) 0)
        (bind _collider (`self.collider`)
          (:`then`
            (`|SpawnActorFromClass` "/Game/Blueprints/Hit_Status_Popup_BP.Hit_Status_Popup_BP_C" (`KismetMathLibrary.MakeTransform` (`SceneComponent.K2_GetComponentLocation` _collider)) "Undefined" "MultiplyWithRoot" null (`local.status`) null))
          (:`else`))))))

(fn `on hit material `
  (params (`in value` :type "Float (double-precision)"))
  (bind _body_ (`self.body `))
  (bind _returnvalue (`PrimitiveComponent.CreateDynamicMaterialInstance` _body_ 0 (`PrimitiveComponent.GetMaterial` _body_ 0) "None"))
  (`MaterialInstanceDynamic.SetScalarParameterValue` _returnvalue "wind_intensity" (`local.in value`)))

(fn `set material as per element color`
  (bind _body_ (`self.body `))
  (`|ExecutionSequence`
    (:`then_0`
      (bind _returnvalue (`PrimitiveComponent.CreateDynamicMaterialInstance` _body_ 0 (`PrimitiveComponent.GetMaterial` _body_ 0) "None"))
      (`MaterialInstanceDynamic.SetVectorParameterValue` _returnvalue "color" (`KismetMathLibrary.Conv_ColorToLinearColor` (`/Game/Blueprints/Components/Element_Assignment_Component.selected element color` (`self.Element_Assignment_Component`)))))))

(fn `UserConstructionScript`)