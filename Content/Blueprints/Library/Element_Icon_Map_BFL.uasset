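; Blueprint function library that supplies UI lookup tables for the seven elements (Pyro, Hydro, Cryo, Electro, Anemo, Geo, Dendro).
; GetElementIconMap rebuilds and returns a map from uppercase element name to that element's UI icon material.
; GetElementColorMap does the same for colors, pulling each value from a freshly made ColorList struct.
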(fn `get element color map`
  (returns (`return color map` :type "Map of String to Color Structure"))
  (locals (`color map` :type "Map of String to Color Structure") (`temp color list` :type "/Game/DataTypes/Color_List Structure"))
  (`|ExecutionSequence`
    (:`then_0`
      (`BlueprintMapLibrary.Map_Clear` (`local.color map`))
      (bind _output_get (set `local.temp color list` (make `/Game/DataTypes/Color_List` (struct :`A` 1))))
      (bind (_immune _hydro _dendro _anemo _pyro _electro _geo _cryo) (break `/Game/DataTypes/Color_List` _output_get))
      (`BlueprintMapLibrary.Map_Add` (`local.color map`) "HYDRO" _hydro)
      (`BlueprintMapLibrary.Map_Add` (`local.color map`) "DENDRO" _dendro)
      (`BlueprintMapLibrary.Map_Add` (`local.color map`) "ANEMO" _anemo)
      (`BlueprintMapLibrary.Map_Add` (`local.color map`) "PYRO" _pyro)
      (`BlueprintMapLibrary.Map_Add` (`local.color map`) "ELECTRO" _electro)
      (`BlueprintMapLibrary.Map_Add` (`local.color map`) "GEO" _geo)
      (`BlueprintMapLibrary.Map_Add` (`local.color map`) "CRYO" _cryo))
    (:`then_1`
      (return (`local.color map`)))))

(fn `get element icon map`
  (returns (`return element icon map` :type "Map of String to Material Object Reference"))
  (locals (temp :type "Map of String to Material Object Reference"))
  (`|ExecutionSequence`
    (:`then_0`
      (`BlueprintMapLibrary.Map_Clear` (`local.temp`))
      (`BlueprintMapLibrary.Map_Add` (`local.temp`) "PYRO" "/Game/My_Textures/logo/Pyro_Icon_UI_Material.Pyro_Icon_UI_Material")
      (`BlueprintMapLibrary.Map_Add` (`local.temp`) "HYDRO" "/Game/My_Textures/logo/Hydro_Icon_UI_Material.Hydro_Icon_UI_Material")
      (`BlueprintMapLibrary.Map_Add` (`local.temp`) "CRYO" "/Game/My_Textures/logo/Cryo_Icon_UI_Material.Cryo_Icon_UI_Material")
      (`BlueprintMapLibrary.Map_Add` (`local.temp`) "ELECTRO" "/Game/My_Textures/logo/Electro_Icon_UI_Material.Electro_Icon_UI_Material")
      (`BlueprintMapLibrary.Map_Add` (`local.temp`) "ANEMO" "/Game/My_Textures/logo/Anemo_Icon_UI_Material.Anemo_Icon_UI_Material")
      (`BlueprintMapLibrary.Map_Add` (`local.temp`) "GEO" "/Game/My_Textures/logo/Geo_Icon_UI_Material.Geo_Icon_UI_Material")
      (`BlueprintMapLibrary.Map_Add` (`local.temp`) "DENDRO" "/Game/My_Textures/logo/Dendro_Icon_UI_Material.Dendro_Icon_UI_Material"))
    (:`then_1`
      (return (`local.temp`)))))