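; A maze paddle-area boundary actor that shows a Niagara effect while a paddle is inside it.
; Box overlap events unhide the Niagara component when a Paddle_BP enters and hide it again when it leaves.
; Two custom events, frontfacing and sidewayfacing, orient the effect by setting its facing vector parameter along the Y or X axis.
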(event `front facing`
  (`NiagaraComponent.SetVariableVec3` (`self.Niagara`) "my_facing_vector" (0.0 1.0 0.0)))

(event `sideway facing`
  (`NiagaraComponent.SetVariableVec3` (`self.Niagara`) "my_facing_vector" (1.0 0.0 0.0)))

(event `self.Box.OnComponentBeginOverlap`
  (params (OverlappedComponent :type "PrimitiveComponent Object Reference") (OtherActor :type "Actor Object Reference") (OtherComp :type "PrimitiveComponent Object Reference") (OtherBodyIndex :type Integer) (bFromSweep :type Boolean) (SweepResult :type "HitResult Structure (by ref)"))
  (cast `/Game/Blueprints/Maze/Paddle_BP` OtherActor)
  (`SceneComponent.SetHiddenInGame` (`self.Niagara`) false false))

(event `self.Box.OnComponentEndOverlap`
  (params (OverlappedComponent :type "PrimitiveComponent Object Reference") (OtherActor :type "Actor Object Reference") (OtherComp :type "PrimitiveComponent Object Reference") (OtherBodyIndex :type Integer))
  (cast `/Game/Blueprints/Maze/Paddle_BP` OtherActor)
  (`SceneComponent.SetHiddenInGame` (`self.Niagara`) true false))

(fn `UserConstructionScript`)