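; Maze actor for a paddle game that builds the play field and moves the paddle within it.
; On BeginPlay it registers with the player character, spawns boundary pieces around the paddle area, configures left, right and front limit child actors, and develops the obstacle grid.
; Tick retries caching the paddle config until valid, then applies sensitivity-scaled motion input as clamped relative movement while control is enabled, triggering movement VFX when the position changes.
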(event `self.ReceiveBeginPlay`
  (`|ExecutionSequence`
    (:`then_1`
      (bind _asgameplay_character_bp (cast `/Game/Blueprints/Gameplay_Character_BP` (`GameplayStatics.GetPlayerCharacter` 0)))
      (set `/Game/Blueprints/Gameplay_Character_BP.maze` self _asgameplay_character_bp))
    (:`then_2`
      (`self.make boundry`))
    (:`then_3`
      (bind _asobstacle_grid_bp (cast `/Game/Blueprints/Obstacles/Obstacle_Grid_BP` (`ChildActorComponent.ChildActor` (`self.obstacle grid child actor`))))
      (`/Game/Blueprints/Obstacles/Obstacle_Grid_BP.develope grid` _asobstacle_grid_bp))))

(event `self.ReceiveTick`
  (params (DeltaSeconds :type "Float (single-precision)"))
  (`|ExecutionSequence`
    (:`then_0`
      (`/Engine/EditorBlueprintResources/StandardMacros.DoOnce` false :!label _label
        (:`Completed`
          (bind _aspaddle_bp (cast `/Game/Blueprints/Maze/Paddle_BP` (`ChildActorComponent.ChildActor` (`self.Paddle`))))
          (bind _my_config (`/Game/Blueprints/Maze/Paddle_BP.my config` _aspaddle_bp)
            (:`then`
              (set `self.paddle config` _my_config))
            (:`else`
              (`/Game/Blueprints/Maze/Paddle_BP.fetch config` _aspaddle_bp)
              (goto _label :!via `Reset`))))))
    (:`then_1`
      (`self.handle paddle movement`))))

(fn `handle paddle movement`
  (locals (`temp ` :type "Vector Structure"))
  (bind (_my_motion_input_x _my_motion_input_y) (`KismetMathLibrary.BreakVector` (`self.my motion input`)))
  (bind _paddle (`self.Paddle`))
  (bind (_relativelocation_x _relativelocation_y _relativelocation_z) (`KismetMathLibrary.BreakVector` (`SceneComponent.RelativeLocation` (`self.Paddle`))))
  (if (`self.can control `)
    (`|ExecutionSequence`
      (:`then_0`
        (bind _paddle_config (`self.paddle config`)
          (:`then`
            (bind _sensitivity (`/Game/Blueprints/Save_Game/Paddle_Config_Save_Game_BP.sensitivity` _paddle_config))
            (set `local.temp ` (`KismetMathLibrary.MakeVector` (`KismetMathLibrary.FClamp` (+ (* _my_motion_input_y (* _sensitivity -3)) _relativelocation_x) -1550.0 -25.0) (`KismetMathLibrary.FClamp` (+ _relativelocation_y (* _my_motion_input_x (* _sensitivity 3))) 0.0 150.0) _relativelocation_z)))
          (:`else`)))
      (:`then_1`
        (if (not (`KismetMathLibrary.EqualExactly_VectorVector` (`self.paddle old location`) (`local.temp `)))
          (`SceneComponent.K2_SetRelativeLocation` _paddle (`local.temp `) false false)
          (bind _aspaddle_bp (cast `/Game/Blueprints/Maze/Paddle_BP` (`ChildActorComponent.ChildActor` _paddle)))
          (`ActorComponent.Activate` (`/Game/Blueprints/Maze/Paddle_BP.movement vfx` _aspaddle_bp) true)))
      (:`then_2`
        (set `self.paddle old location` (`local.temp `))))))

(fn `make boundry`
  (`|ExecutionSequence`
    (:`then_0`
      ;[1 1 1] left and right boundry
      (for _index (range 10)
        (bind _returnvalue (+ (`self.K2_GetActorLocation`) (`KismetMathLibrary.MakeVector` 0.0 (* _index 40))))
        (bind _returnvalue_2 (`|SpawnActorFromClass` "/Game/Blueprints/Maze/Paddle_Area_Boundry_BP.Paddle_Area_Boundry_BP_C" (`KismetMathLibrary.MakeTransform` _returnvalue) "Undefined" "MultiplyWithRoot" null null))
        (`/Game/Blueprints/Maze/Paddle_Area_Boundry_BP.sideway facing` _returnvalue_2)
        (bind _returnvalue_3 (`|SpawnActorFromClass` "/Game/Blueprints/Maze/Paddle_Area_Boundry_BP.Paddle_Area_Boundry_BP_C" (`KismetMathLibrary.MakeTransform` (+ _returnvalue (-2000.0 0.0 0.0))) "Undefined" "MultiplyWithRoot" null null))
        (`/Game/Blueprints/Maze/Paddle_Area_Boundry_BP.sideway facing` _returnvalue_3)))
    (:`then_1`
      ;[1 1 1] front and back boundry
      (for _index_2 (range 51)
        (bind _returnvalue_4 (+ (`self.K2_GetActorLocation`) (`KismetMathLibrary.MakeVector` (* _index_2 -40) -40.0)))
        (bind _returnvalue_5 (`|SpawnActorFromClass` "/Game/Blueprints/Maze/Paddle_Area_Boundry_BP.Paddle_Area_Boundry_BP_C" (`KismetMathLibrary.MakeTransform` _returnvalue_4) "Undefined" "MultiplyWithRoot" null null))
        (`/Game/Blueprints/Maze/Paddle_Area_Boundry_BP.front facing` _returnvalue_5)
        (bind _returnvalue_6 (`|SpawnActorFromClass` "/Game/Blueprints/Maze/Paddle_Area_Boundry_BP.Paddle_Area_Boundry_BP_C" (`KismetMathLibrary.MakeTransform` (+ _returnvalue_4 (0.0 250.0 0.0))) "Undefined" "MultiplyWithRoot" null null))
        (`/Game/Blueprints/Maze/Paddle_Area_Boundry_BP.front facing` _returnvalue_6)))
    (:`then_2`
      (bind _aslimit_parent_bp (cast `/Game/Blueprints/Limit/Limit_Parent_BP` (`ChildActorComponent.ChildActor` (`self.limit child actor left`))))
      (set `/Game/Blueprints/Limit/Limit_Parent_BP.is column` true _aslimit_parent_bp)
      (`/Game/Blueprints/Limit/Limit_Parent_BP.develope limit` _aslimit_parent_bp)
      (`/Game/Blueprints/Limit/Limit_Parent_BP.parent is left wall` _aslimit_parent_bp))
    (:`then_3`
      (bind _aslimit_parent_bp_2 (cast `/Game/Blueprints/Limit/Limit_Parent_BP` (`ChildActorComponent.ChildActor` (`self.limit child actor right`))))
      (set `/Game/Blueprints/Limit/Limit_Parent_BP.is column` true _aslimit_parent_bp_2)
      (`/Game/Blueprints/Limit/Limit_Parent_BP.develope limit` _aslimit_parent_bp_2)
      (`/Game/Blueprints/Limit/Limit_Parent_BP.parent is right wall` _aslimit_parent_bp_2))
    (:`then_4`
      (bind _aslimit_parent_bp_3 (cast `/Game/Blueprints/Limit/Limit_Parent_BP` (`ChildActorComponent.ChildActor` (`self.limit child actor front`))))
      (set `/Game/Blueprints/Limit/Limit_Parent_BP.is column` false _aslimit_parent_bp_3)
      (`/Game/Blueprints/Limit/Limit_Parent_BP.develope limit` _aslimit_parent_bp_3)
      (`/Game/Blueprints/Limit/Limit_Parent_BP.parent is front wall` _aslimit_parent_bp_3))))

(fn `UserConstructionScript`)