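; Blast actor that expands a sphere and notifies enemies and ball projectiles caught inside it.
; On BeginPlay a timeline grows the Sphere collision radius along a curve, updating overlaps as it goes.
; When the timeline finishes, it sends HitByBlastMessage through Blast_BPI to overlapping Enemy_Base_BP and Ball_Projectile_BP actors that implement the interface, then destroys itself.
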(event `self.ReceiveBeginPlay`
  (bind (_direction _radius_track) (`Timeline|radius timeline`)
    (:`Update`
      (`SphereComponent.SetSphereRadius` (`self.Sphere`) _radius_track true))
    (:`Finished`
      (`|ExecutionSequence`
        (:`then_0`
          (for _array_element (`PrimitiveComponent.GetOverlappingActors` (`self.Sphere`) "/Game/Blueprints/Obstacles/Enemy/Enemy_Base_BP.Enemy_Base_BP_C")
            (if (`KismetSystemLibrary.DoesImplementInterface` _array_element "/Game/Blueprints/Interface/Blast_BPI.Blast_BPI_C")
              (message `/Game/Blueprints/Interface/Blast_BPI.hit by blast` _array_element (make `/Game/DataTypes/Blast_Damage_Configuration_Data_Structure` true)))))
        (:`then_1`
          (for _array_element_2 (`PrimitiveComponent.GetOverlappingActors` (`self.Sphere`) "/Game/Blueprints/Ball/Ball_Projectile_BP.Ball_Projectile_BP_C")
            (if (`KismetSystemLibrary.DoesImplementInterface` _array_element_2 "/Game/Blueprints/Interface/Blast_BPI.Blast_BPI_C")
              (message `/Game/Blueprints/Interface/Blast_BPI.hit by blast` _array_element_2 (make `/Game/DataTypes/Blast_Damage_Configuration_Data_Structure` true)))))
        (:`then_2`
          (`self.K2_DestroyActor`))))))

(fn `UserConstructionScript`)