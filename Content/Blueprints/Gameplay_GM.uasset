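; Gameplay game mode that sets up the selected mode and stage by rebuilding its saved maze on the obstacle grid.
; On BeginPlay it caches the layout data, grid and visualizer actors, then async-loads the selection save game.
; On load it pushes the mode info HUD, finds the layout matching mode name and stage, and passes it to the grid.
; A separate function pushes the maze adjustment HUD.
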(event `init refs`
  (`|ExecutionSequence`
    (:`then_1`
      (bind _outactors (`GameplayStatics.GetAllActorsOfClass` "/Game/Blueprints/Save_Data/Mode_Layout_Save_Data_BP.Mode_Layout_Save_Data_BP_C"))
      (set `self.layout save data ref` (`|GetArrayItem` _outactors)))
    (:`then_2`
      (bind _outactors_2 (`GameplayStatics.GetAllActorsOfClass` "/Game/Blueprints/Obstacles/Obstacle_Grid_BP.Obstacle_Grid_BP_C"))
      (set `self.grid ref` (`|GetArrayItem` _outactors_2)))
    (:`then_3`
      (bind _outactors_3 (`GameplayStatics.GetAllActorsOfClass` "/Game/Blueprints/Sound/Audio_Visualizer_BP.Audio_Visualizer_BP_C"))
      (set `self.visualizer ref` (`|GetArrayItem` _outactors_3)))))

(event `self.ReceiveBeginPlay`
  (`parent.ReceiveBeginPlay`)
  (`self.init refs`)
  (`self.fetch mode`))

(event `fetch mode`
  (bind _savegame (`AsyncActionHandleSaveGame.AsyncLoadGameFromSlot` (`|GetEnumeratorNameAsString` (enumliteral `/Game/DataTypes/Save_Game_Slot_Names_ENUM` "NewEnumerator1")))
    (:`Completed`
      (bind _asgame_mode_and_stage_selected_save_game_bp (cast `/Game/Blueprints/Save_Game/Game_Mode_And_Stage_Selected_Save_Game_BP` _savegame))
      (set `self.Name Enum` (`/Game/Blueprints/Save_Game/Game_Mode_And_Stage_Selected_Save_Game_BP.name enum` _asgame_mode_and_stage_selected_save_game_bp))
      (set `self.Stage` (`/Game/Blueprints/Save_Game/Game_Mode_And_Stage_Selected_Save_Game_BP.stage` _asgame_mode_and_stage_selected_save_game_bp))
      (`self.push hud` "/Game/UI/Blueprints/Mode_Info/Begin_Play_Mode_Info_Main_Widget_BP.Begin_Play_Mode_Info_Main_Widget_BP_C")
      (`self.populate maze`))))

(fn `populate maze`
  (locals (`mode layout index` :type Integer :default 0))
  (bind (_output_gamemodename _output_stage _output_gridlayout) (break `/Game/DataTypes/GamePlay/Mode_Layout_Data_Structure` (`|GetArrayItem` (`/Game/Blueprints/Save_Data/Mode_Layout_Save_Data_BP.mode layout` (`self.layout save data ref`)) (`self.selected mode layout index`))))
  (`|ExecutionSequence`
    (:`then_0`
      (if (== (`self.selected mode layout index`) -1)
        (for (_array_element _array_index) (`/Game/Blueprints/Save_Data/Mode_Layout_Save_Data_BP.mode layout` (`self.layout save data ref`))
          (if (and (`KismetStringLibrary.EqualEqual_StrStr` (`|GetEnumeratorNameAsString` (`self.Name Enum`)) (break `/Game/DataTypes/GamePlay/Mode_Layout_Data_Structure` _array_element)) (== (`.stage_9_423DD46440530A1DBDE0268320844CAA` (break `/Game/DataTypes/GamePlay/Mode_Layout_Data_Structure` _array_element)) (`self.Stage`)))
            (set `self.selected mode layout index` _array_index)
            (break)))))
    (:`then_1`
      (`/Game/Blueprints/Obstacles/Obstacle_Grid_BP.develope grid from memory` (`self.grid ref`) _output_gridlayout))))

(fn `push adjustment hud`
  (`self.push hud` "/Game/UI/Blueprints/Adjustment/Maze_Main_Widget_BP.Maze_Main_Widget_BP_C"))

(fn `UserConstructionScript`)