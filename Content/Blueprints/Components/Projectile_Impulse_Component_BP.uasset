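; Component on Ball_Projectile_BP that drives the ball's physics velocity, launching it along Y at BeginPlay.
; HandleVelocity picks random-sign X/Y velocity of fixed magnitude, which Tick re-applies whenever the squared speed drifts.
; ImpulseAbsorbed, meant for the ball's hit handler, halves the magnitude of new picks until a Duration timer expires.
; HandleGamePause, meant for the gameplay helper component, saves velocity and disables physics, restoring both on resume.
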(event `impulse absorbed`
  ;[1 1 1] called via handle hit function  of ball projectile
  (set `self.is impulse absorbed` true)
  (set `self.count` 0.0))

(event `handle velocity`
  ;[1 1 1] called via handle hit function  of ball projectile
  (bind _collider (`self.Collider`)
    (:`then`
      (if (`SceneComponent.IsSimulatingPhysics` _collider "None")
        (bind _collider_2 (`self.Collider`)
          (:`then`
            (bind _output_get (set `self.velocity made` (`KismetMathLibrary.MakeVector` (`self.get positive or negative magnitude `) (`self.get positive or negative magnitude `))))
            (`PrimitiveComponent.SetAllPhysicsLinearVelocity` _collider_2 _output_get false))
          (:`else`))))
    (:`else`)))

(event `handle counter`
  ;[1 1 1] used to mimic impulse absorbed
  (if (`self.is impulse absorbed`)
    (bind _output_get (set `self.count` (+ (`self.count`) (`GameplayStatics.GetWorldDeltaSeconds`))))
    (if (> _output_get (`self.duration`))
      (set `self.is impulse absorbed` false)
      (set `self.count` 0.0))))

(event `handle game pause`
  ;[1 1 1] call it via gameplay helper component only
  (if (`/Game/Blueprints/Components/Gameplay_Helper_Component_BP.Do Pause` (`/Game/Blueprints/Gameplay_GM.Gameplay_Helper_Component_BP` (`self.As Gameplay GM`)))
    (`/Engine/EditorBlueprintResources/StandardMacros.DoOnce` false :!label _label
      (:`Completed`
        (`self.on game pause`)))
    (else
      (`self.on game continue`)
      (goto _label :!via `Reset`))))

(event `self.ReceiveTick`
  (params (DeltaSeconds :type "Float (single-precision)"))
  (if (not (`/Game/Blueprints/Components/Gameplay_Helper_Component_BP.Do Pause` (`/Game/Blueprints/Gameplay_GM.Gameplay_Helper_Component_BP` (`self.As Gameplay GM`))))
    (`|ExecutionSequence`
      (:`then_0`
        (`self.handle counter`))
      (:`then_1`
        (`self.match velocity`)))))

(event `self.ReceiveBeginPlay`
  (`|ExecutionSequence`
    (:`then_0`
      (bind _asgameplay_gm (cast `/Game/Blueprints/Gameplay_GM` (`GameplayStatics.GetGameMode`)))
      (set `self.As Gameplay GM` _asgameplay_gm))
    (:`then_1`
      (bind _asball_projectile_bp (cast `/Game/Blueprints/Ball/Ball_Projectile_BP` (`self.GetOwner`)))
      (bind _output_get (set `self.Collider` (`/Game/Blueprints/Ball/Ball_Base_BP.collider` _asball_projectile_bp)))
      (`PrimitiveComponent.SetAllPhysicsLinearVelocity` _output_get (0.0 1500.0 0.0) false))))

(fn `get positive or negative magnitude `
  (returns (ReturnValue :type "Float (double-precision)"))
  (if (`self.is impulse absorbed`)
    (if (> (`KismetMathLibrary.RandomFloat`) 0.5)
      (return (* (`self.magnitude`) 0.5))
      (else
        (return (* (`self.magnitude`) -0.5))))
    (elif (> (`KismetMathLibrary.RandomFloat`) 0.5)
      (return (`self.magnitude`))
      (else
        (return (* (`self.magnitude`) -1.0))))))

(fn `match velocity`
  (bind _velocity_made (`self.velocity made`))
  (if (!= (`KismetMathLibrary.VSize` (`self.velocity made`)) 0.0)
    (bind _collider (`self.Collider`)
      (:`then`
        (if (!= (`KismetMathLibrary.VSizeSquared` (`SceneComponent.GetComponentVelocity` _collider)) (`KismetMathLibrary.VSizeSquared` _velocity_made))
          (`PrimitiveComponent.SetAllPhysicsLinearVelocity` _collider _velocity_made false)))
      (:`else`))))

(fn `on game continue`
  (bind _collider (`self.Collider`)
    (:`then`
      (`PrimitiveComponent.SetSimulatePhysics` _collider true)
      (bind _collider_2 (`self.Collider`)
        (:`then`
          (`PrimitiveComponent.SetAllPhysicsLinearVelocity` _collider_2 (`self.before velocity`) false))
        (:`else`)))
    (:`else`)))

(fn `on game pause`
  (bind _collider (`self.Collider`)
    (:`then`
      (set `self.before velocity` (`SceneComponent.GetComponentVelocity` _collider))
      (bind _collider_2 (`self.Collider`)
        (:`then`
          (`PrimitiveComponent.SetSimulatePhysics` _collider_2 false))
        (:`else`)))
    (:`else`)))