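; Enemy 5 is an element-colored enemy obstacle that cracks as it loses health and spawns a blast when killed.
; It tints its body material, crack child actor and Niagara effects by element, while a timeline animates body height.
; Projectile and blast hits run parent logic, spawn reaction-gated popups and VFX, then use HP percent to drive material, cracks and escaping particles.
; Death spawns Blast_BP and colored VFX, plays a sound and destroys the actor.
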(event `handle timeline`
  (if (and (not (`self.event on kill`)) (`self.can play timeline`))
    (bind (_direction _z_track) (`Timeline|body timeline` :!label _label)
      (:`Update`
        (`SceneComponent.K2_SetRelativeLocation` (`self.body`) (`KismetMathLibrary.MakeVector` 0.0 0.0 _z_track) false false)))
    (else
      (goto _label :!via `Stop`))))

(event `/Game/Blueprints/Interface/Initialization_BPI.init again`
  (params (`selected element name` :type String) (`in memory` :type Boolean))
  (`parent.init again` `selected element name` false)
  (`|ExecutionSequence` :!label _label_2
    (:`then_0`
      (`self.set material as per element color`)
      (`self.update material on hit`))
    (:`then_1`
      (`self.set vfx as pr element color`))
    (:`then_2`
      (`self.handle timeline`))))

(event `self.ReceiveBeginPlay`
  (`parent.ReceiveBeginPlay`)
  (goto _label_2))

(event `/Game/Blueprints/Interface/Blast_BPI.hit by blast`
  (params (`blast configuration` :type "/Game/DataTypes/Blast_Damage_Configuration_Data_Structure Structure"))
  (`parent.hit by blast` `blast configuration`)
  (`|ExecutionSequence`
    (:`then_0`
      (`self.handle spawning of vfx` "Explosive Impact" true))
    (:`then_1`
      (`self.update material on hit`))
    (:`then_2`
      (`self.handle cracking`))
    (:`then_3`
      (`self.update vfx on hit`))))

(event `/Game/Blueprints/Interface/Ball_Projectile_On_Hit_BPI.hit by projectile`
  (params (`damage configuration` :type "/Game/DataTypes/Projectile_Damage_Configuration_Data_Structure Structure") (`projectile element name` :type "String (by ref)"))
  (`parent.hit by projectile` `damage configuration` `projectile element name`)
  (`|ExecutionSequence`
    (:`then_0`
      (`self.handle spawning of vfx` "Building Charge" true))
    (:`then_1`
      (`self.update material on hit`))
    (:`then_2`
      (`self.handle cracking`))
    (:`then_3`
      (`self.update vfx on hit`))))

(event `/Game/Blueprints/Interface/Kill_BPI.handle kill`
  (`parent.handle kill`)
  (`|ExecutionSequence`
    (:`then_0`
      (`|SpawnActorFromClass` "/Game/Blueprints/Obstacles/Enemy/Blast_BP.Blast_BP_C" (`KismetMathLibrary.MakeTransform` (`SceneComponent.K2_GetComponentLocation` (`self.collider`))) "Undefined" "MultiplyWithRoot" null null))
    (:`then_1`
      (`|SpawnActorFromClass` "/Game/Blueprints/VFX/E5_On_Kill_VFX_BP.E5_On_Kill_VFX_BP_C" (`KismetMathLibrary.MakeTransform` (`SceneComponent.K2_GetComponentLocation` (`self.collider`))) "Undefined" "MultiplyWithRoot" null (`/Game/Blueprints/Components/Element_Assignment_Component.selected element color` (`self.Element_Assignment_Component`)) null))
    (:`then_2`
      (`GameplayStatics.PlaySound2D` "/Game/Audio/cue/E5_Explosion_Cue.E5_Explosion_Cue" 1.0 1.0 0.0 null null))
    (:`then_3`
      (set `self.event on kill` true))
    (:`then_4`
      (`self.handle timeline`))
    (:`then_5`
      (`self.K2_DestroyActor`))))

(fn `handle cracking`
  (bind _cracked_body_child_actor (`self.cracked body child actor`)
    (:`then`
      (bind _ase5_body_crack_bp (cast `/Game/Blueprints/Obstacles/Enemy/E5_Body_Crack_BP` (`ChildActorComponent.ChildActor` _cracked_body_child_actor)))
      (`/Game/Blueprints/Obstacles/Enemy/E5_Body_Crack_BP.handle cracks using hp percent` _ase5_body_crack_bp (`self.my hp percent`)))
    (:`else`)))

(fn `handle spawning of vfx`
  (params (status :type Text :default "NSLOCTEXT(\"[7EA2782040D8599571FD9270AD94881C]\", \"E76A475E486EBA99CB4C3DBA908CB061\", \"Default Status\")") (particle :type Boolean))
  (`|ExecutionSequence`
    (:`then_0`
      (if (and (!= (`KismetStringLibrary.Len` (`KismetTextLibrary.Conv_TextToString` (`local.status`))) 0) (`self.reaction occured`))
        (bind _collider (`self.collider`)
          (:`then`
            (`|SpawnActorFromClass` "/Game/Blueprints/Hit_Status_Popup_BP.Hit_Status_Popup_BP_C" (`KismetMathLibrary.MakeTransform` (`SceneComponent.K2_GetComponentLocation` _collider)) "Undefined" "MultiplyWithRoot" null (`local.status`) null))
          (:`else`))))
    (:`then_1`
      (if (and (`local.particle`) (`self.reaction occured`))
        (bind _collider_2 (`self.collider`)
          (:`then`
            (bind _element_assignment_component (`self.Element_Assignment_Component`)
              (:`then`
                (`|SpawnActorFromClass` "/Game/Blueprints/VFX/Enemy_5_On_Hit_VFX_BP.Enemy_5_On_Hit_VFX_BP_C" (`KismetMathLibrary.MakeTransform` (- (`SceneComponent.K2_GetComponentLocation` _collider_2) (0.0 0.0 100.0))) "Undefined" "MultiplyWithRoot" null (`/Game/Blueprints/Components/Element_Assignment_Component.selected element color` _element_assignment_component) null))
              (:`else`)))
          (:`else`))))))

(fn `set material as per element color`
  (bind _body (`self.body`))
  (bind _selected_element_color (`/Game/Blueprints/Components/Element_Assignment_Component.selected element color` (`self.Element_Assignment_Component`)))
  (`|ExecutionSequence`
    (:`then_0`
      (bind _returnvalue (`PrimitiveComponent.CreateDynamicMaterialInstance` _body 0 (`PrimitiveComponent.GetMaterial` _body 0) "None"))
      (bind _output_get (set `self.body dm` _returnvalue))
      (`MaterialInstanceDynamic.SetVectorParameterValue` _output_get "color" (`KismetMathLibrary.Conv_ColorToLinearColor` _selected_element_color)))
    (:`then_1`
      (bind _ase5_body_crack_bp (cast `/Game/Blueprints/Obstacles/Enemy/E5_Body_Crack_BP` (`ChildActorComponent.ChildActor` (`self.cracked body child actor`))))
      (`/Game/Blueprints/Obstacles/Enemy/E5_Body_Crack_BP.set material as per element color` _ase5_body_crack_bp _selected_element_color))))

(fn `set vfx as pr element color`
  (bind _returnvalue (* (`KismetMathLibrary.Conv_ColorToLinearColor` (`/Game/Blueprints/Components/Element_Assignment_Component.selected element color` (`self.Element_Assignment_Component`))) (struct :`R` 100.0 :`G` 100.0 :`B` 100.0 :`A` 1.0)))
  (`|ExecutionSequence`
    (:`then_0`
      (`NiagaraComponent.SetVariableLinearColor` (`self.body vfx`) "element_color" _returnvalue))
    (:`then_1`
      (`NiagaraComponent.SetVariableLinearColor` (`self.escaping particles vfx`) "element_color" _returnvalue))))

(fn `update material on hit`
  (`MaterialInstanceDynamic.SetScalarParameterValue` (`self.body dm`) "hp_percent" (`KismetMathLibrary.Conv_IntToDouble` (`self.my hp percent`))))

(fn `update vfx on hit`
  (`|ExecutionSequence`
    (:`then_0`
      (bind _escaping_particles_vfx (`self.escaping particles vfx`)
        (:`then`
          (`NiagaraComponent.SetVariableFloat` _escaping_particles_vfx "count" (`KismetMathLibrary.Conv_IntToDouble` (- 100 (`self.my hp percent`)))))
        (:`else`)))))

(fn `UserConstructionScript`)