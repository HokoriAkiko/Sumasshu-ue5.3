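; Maze floor spawner that builds the game's grid floor and its surrounding audio visualization border on BeginPlay.
; Nested loops spawn Floor_Shape_BP across the configured X/Y range, then Audio_Visualization_Shape_BP in a band beyond EndY and two hard-coded side strips.
; MakeLocationVector maps indices to 200-unit spacing with X negated, and each piece attaches to the spawner's root.
; Once spawning finishes, it calls InitVisualizer on every Audio_Visualizer_BP in the level.
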(event `self.ReceiveBeginPlay`
  (bind _end_y (`self.end y`))
  (`|ExecutionSequence`
    (:`then_0`
      ;[1 1 1] This is the main game floor area
      (for _index (range (`self.start y`) (+ (`self.end y`) 1))
        (for _index_2 (range (`self.start x`) (+ (`self.end x`) 1))
          (bind _returnvalue (`|SpawnActorFromClass` "/Game/Blueprints/World_Cube/Shape/Floor_Shape_BP.Floor_Shape_BP_C" (`KismetMathLibrary.MakeTransform` (`self.make location vector` _index_2 _index)) "Undefined" "MultiplyWithRoot" null (0.0 0.0 1.0) null))
          (`self.K2_AttachToComponent` _returnvalue (`self.DefaultSceneRoot`) "None" "KeepRelative" "KeepRelative" "KeepRelative" true))))
    (:`then_1`
      ;[1 1 1] This is the visualization mesh on top of the floor
      (for _index_3 (range (+ _end_y 1) (+ (+ _end_y 4) 1))
        (for _index_4 (range (`self.start x`) (+ (`self.end x`) 1))
          (bind _returnvalue_2 (`|SpawnActorFromClass` "/Game/Blueprints/World_Cube/Shape/Audio_Visualization_Shape_BP.Audio_Visualization_Shape_BP_C" (`KismetMathLibrary.MakeTransform` (`self.make location vector` _index_4 _index_3)) "Undefined" "MultiplyWithRoot" null null))
          (`self.K2_AttachToComponent` _returnvalue_2 (`self.DefaultSceneRoot`) "None" "KeepRelative" "KeepRelative" "KeepRelative" true))))
    (:`then_2`
      (for _index_5 (range (`self.start y`) (+ (+ (`self.end y`) 3) 1))
        (for _index_6 (range -5 -1)
          (bind _returnvalue_3 (`|SpawnActorFromClass` "/Game/Blueprints/World_Cube/Shape/Audio_Visualization_Shape_BP.Audio_Visualization_Shape_BP_C" (`KismetMathLibrary.MakeTransform` (`self.make location vector` _index_6 _index_5)) "Undefined" "MultiplyWithRoot" null null))
          (`self.K2_AttachToComponent` _returnvalue_3 (`self.DefaultSceneRoot`) "None" "KeepRelative" "KeepRelative" "KeepRelative" true))))
    (:`then_3`
      (for _index_7 (range (`self.start y`) (+ (+ (`self.end y`) 3) 1))
        (for _index_8 (range 11 16)
          (bind _returnvalue_4 (`|SpawnActorFromClass` "/Game/Blueprints/World_Cube/Shape/Audio_Visualization_Shape_BP.Audio_Visualization_Shape_BP_C" (`KismetMathLibrary.MakeTransform` (`self.make location vector` _index_8 _index_7)) "Undefined" "MultiplyWithRoot" null null))
          (`self.K2_AttachToComponent` _returnvalue_4 (`self.DefaultSceneRoot`) "None" "KeepRelative" "KeepRelative" "KeepRelative" true))))
    (:`then_4`
      (bind _outactors (`GameplayStatics.GetAllActorsOfClass` "/Game/Blueprints/Sound/Audio_Visualizer_BP.Audio_Visualizer_BP_C"))
      (for _array_element _outactors
        (`/Game/Blueprints/Sound/Audio_Visualizer_BP.init visualizer` _array_element)))))

(fn `make location vector`
  (params (`x index` :type Integer) (`y index` :type Integer))
  (returns (`return vector` :type "Vector Structure"))
  (return (`KismetMathLibrary.MakeVector` (`KismetMathLibrary.Conv_IntToDouble` (* `x index` -200)) (`KismetMathLibrary.Conv_IntToDouble` (* `y index` 200)))))

(fn `UserConstructionScript`)