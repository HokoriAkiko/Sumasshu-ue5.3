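; Body crack overlay for the E5 enemy obstacle that shows damage as its health drops.
; On BeginPlay it gives each child component a random rotation.
; A health-percent event reveals four crack components at descending thresholds and raises audio volume as health falls.
; A separate function tints the child meshes to an element color through dynamic material instances.
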(event `self.ReceiveBeginPlay`
  (for _array_element (`SceneComponent.GetChildrenComponents` (`self.DefaultSceneRoot`) false)
    (`SceneComponent.K2_SetRelativeRotation` _array_element (`KismetMathLibrary.RandomRotator` true) false false)))

(event `handle cracks using hp percent`
  (params (`hp percent` :type Integer))
  (bind _1 (`self.1`))
  (bind _2 (`self.2`))
  (bind _3 (`self.3`))
  (bind _4 (`self.4`))
  (`|ExecutionSequence`
    (:`then_0`
      (if (<= `hp percent` 80)
        ;[1 1 1] Visible
        (`SceneComponent.SetHiddenInGame` _1 false false)
        (else
          ;[1 1 1] Hidden
          (`SceneComponent.SetHiddenInGame` _1 true false))))
    (:`then_1`
      (if (<= `hp percent` 60)
        (`SceneComponent.SetHiddenInGame` _2 false false)
        (else
          (`SceneComponent.SetHiddenInGame` _2 true false))))
    (:`then_2`
      (if (<= `hp percent` 40)
        (`SceneComponent.SetHiddenInGame` _3 false false)
        (else
          (`SceneComponent.SetHiddenInGame` _3 true false))))
    (:`then_3`
      (if (<= `hp percent` 20)
        (`SceneComponent.SetHiddenInGame` _4 false false)
        (else
          (`SceneComponent.SetHiddenInGame` _4 true false))))
    (:`then_4`
      (`AudioComponent.SetVolumeMultiplier` (`self.Audio`) (- 1.0 (* (`KismetMathLibrary.Conv_IntToDouble` `hp percent`) 0.01))))))

(fn `set material as per element color`
  (params (`my color` :type "Color Structure"))
  (for _array_element (`SceneComponent.GetChildrenComponents` (`self.DefaultSceneRoot`) false)
    (bind _asstatic_mesh_component (cast `StaticMeshComponent` _array_element))
    (bind _returnvalue (`PrimitiveComponent.CreateDynamicMaterialInstance` _asstatic_mesh_component 0 (`PrimitiveComponent.GetMaterial` _asstatic_mesh_component 0) "None"))
    (`MaterialInstanceDynamic.SetVectorParameterValue` _returnvalue "color" (`KismetMathLibrary.Conv_ColorToLinearColor` (`local.my color`)))))

(fn `UserConstructionScript`)