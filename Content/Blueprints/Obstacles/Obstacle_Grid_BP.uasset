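; Obstacle grid actor that builds a field of obstacles from attached Obstacle_Column_BP actors.
; DevelopeGrid destroys every column actor in the world, then spawns columns spaced along negative X by GapScale, passing rows, obstacle types and spawn probability for each to generate itself.
; FetchGrid captures each attached column's relative transform and layout into an array.
; DevelopeGridFromMemory rebuilds the grid from such a saved layout.
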(event `develope grid`
  (`|ExecutionSequence`
    (:`then_0`
      ;[1 1 1] removing all previously attached child actor components for a fresh new developement
      (bind _outactors (`GameplayStatics.GetAllActorsOfClass` "/Game/Blueprints/Obstacles/Obstacle_Column_BP.Obstacle_Column_BP_C"))
      (for _array_element _outactors
        (`self.K2_DestroyActor` _array_element)))
    (:`then_1`
      ;[1 1 1] handle scaling
      (set `self.multiplier` (+ (-200.0 0.0 0.0) (`KismetMathLibrary.MakeVector` (* (`self.gap scale`) -50)))))
    (:`then_2`
      ;[1 1 1] spawning , attaching and generating column
      (for _index (range (`self.columns`))
        (bind _returnvalue (`|SpawnActorFromClass` "/Game/Blueprints/Obstacles/Obstacle_Column_BP.Obstacle_Column_BP_C" (`KismetMathLibrary.MakeTransform` (* (`self.multiplier`) _index)) "Undefined" "MultiplyWithRoot" null (`self.rows`) (`self.gap scale`) (`self.obstacle types to spawn`) false (`self.spawn probability`) null))
        (`self.K2_AttachToComponent` _returnvalue (`self.DefaultSceneRoot`) "None" "KeepRelative" "KeepRelative" "KeepRelative" true)
        (`/Game/Blueprints/Obstacles/Obstacle_Column_BP.develope column` _returnvalue)))))

(event `develope grid from memory`
  (params (`grid layout` :type "Array of /Game/DataTypes/GamePlay/Grid_Layout_Data_Structure Structure"))
  (`|ExecutionSequence`
    (:`then_0`
      (bind _outactors (`GameplayStatics.GetAllActorsOfClass` "/Game/Blueprints/Obstacles/Obstacle_Column_BP.Obstacle_Column_BP_C"))
      (for _array_element _outactors
        (`self.K2_DestroyActor` _array_element)))
    (:`then_1`
      (for _array_element_2 `grid layout`
        (bind _returnvalue (`|SpawnActorFromClass` :`Class` "/Game/Blueprints/Obstacles/Obstacle_Column_BP.Obstacle_Column_BP_C" :`SpawnTransform` (break `/Game/DataTypes/GamePlay/Grid_Layout_Data_Structure` _array_element_2) :`CollisionHandlingOverride` "Undefined" :`TransformScaleMethod` "MultiplyWithRoot" :`spawn probability` (`self.spawn probability`) :`Instigator` null))
        (`self.K2_AttachToComponent` _returnvalue (`self.DefaultSceneRoot`) "None" "KeepRelative" "KeepRelative" "KeepRelative" true)
        (`/Game/Blueprints/Obstacles/Obstacle_Column_BP.develope column from memory` _returnvalue (`.enemieslayout_7_254C8CDF4FC35ED2C595C683D716046F` (break `/Game/DataTypes/GamePlay/Grid_Layout_Data_Structure` _array_element_2)))))))

(fn `fetch grid `
  (returns (`grid layout` :type "Array of /Game/DataTypes/GamePlay/Grid_Layout_Data_Structure Structure"))
  (locals (`temp grid layout` :type "Array of /Game/DataTypes/GamePlay/Grid_Layout_Data_Structure Structure"))
  (`|ExecutionSequence`
    (:`then_0`
      (for _array_element (`self.GetAttachedActors` true)
        (bind _asobstacle_column_bp (cast `/Game/Blueprints/Obstacles/Obstacle_Column_BP` _array_element))
        (`KismetArrayLibrary.Array_Add` (`local.temp grid layout`) (make `/Game/DataTypes/GamePlay/Grid_Layout_Data_Structure` (`SceneComponent.GetRelativeTransform` (`/Game/Blueprints/Obstacles/Obstacle_Column_BP.DefaultSceneRoot` _asobstacle_column_bp)) (`/Game/Blueprints/Obstacles/Obstacle_Column_BP.fetch column` _asobstacle_column_bp)))))
    (:`then_1`
      (return (`local.temp grid layout`)))))

(fn `UserConstructionScript`)