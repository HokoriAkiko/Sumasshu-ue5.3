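; Main game mode for a maze game that manages settings saves, the HUD stack, total damage and paddle control.
; On BeginPlay it async-loads or creates the settings save, then caches the maze and widget helper actors.
; HUD push, pop and clear edit a class stack, then recreate every widget after garbage collection, with only the top taking input.
; Damage totals go to the gameplay HUD, and the paddle-control flag to the maze.
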(event `save settings`
  (`AsyncActionHandleSaveGame.AsyncSaveGameToSlot` (`self.game settings`) (`|GetEnumeratorNameAsString` (enumliteral `/Game/DataTypes/Save_Game_Slot_Names_ENUM` "NewEnumerator4"))
    (:`Completed`
      (`KismetSystemLibrary.PrintString` "settings saved...."))))

(event `fetch settings`
  (bind _savegame (`AsyncActionHandleSaveGame.AsyncLoadGameFromSlot` (`|GetEnumeratorNameAsString` (enumliteral `/Game/DataTypes/Save_Game_Slot_Names_ENUM` "NewEnumerator4")))
    (:`Completed`
      (bind _assettings_saved_bp (cast `/Game/Blueprints/Save_Game/Settings_Saved_BP` _savegame)
        (:`then`
          (set `self.game settings` _assettings_saved_bp))
        (:`CastFailed`
          (bind _returnvalue (`GameplayStatics.CreateSaveGameObject` "/Game/Blueprints/Save_Game/Settings_Saved_BP.Settings_Saved_BP_C"))
          (set `self.game settings` _returnvalue)))
      (`self.after fetch`))))

(event `after fetch`
  (`|ExecutionSequence`
    (:`then_0`
      (bind _outactors (`GameplayStatics.GetAllActorsOfClass` "/Game/Blueprints/Maze/Maze_BP.Maze_BP_C"))
      (for _array_element _outactors
        (`/Engine/EditorBlueprintResources/StandardMacros.IsValid` _array_element
          (:`Is Valid`
            (set `self.maze ref` _array_element)))))
    (:`then_1`
      (bind _outactors_2 (`GameplayStatics.GetAllActorsOfClass` "/Game/Blueprints/Widget_Helper_BP.Widget_Helper_BP_C"))
      (set `self.widget helper ref` (`|GetArrayItem` _outactors_2)))))

(event `self.ReceiveBeginPlay`
  (`self.fetch settings`))

(event `calculate total damage`
  (params (`incoming damage` :type Integer))
  (set `self.total damage` (+ `incoming damage` (`self.total damage`)))
  (`self.show damage on gameplay hud`))

(fn `clear`
  (params (`after clear class` :type "/Game/UI/Blueprints/Main_HUD_Widget_BP Class Reference"))
  (if (`self.manage huds`)
    (`KismetArrayLibrary.Array_Clear` (`self.hud class stack`))
    (if (`KismetSystemLibrary.IsValidClass` `after clear class`)
      (`KismetArrayLibrary.Array_Add` (`self.hud class stack`) `after clear class`))
    (`self.handle adding to viewport` false)))

(fn `handle adding to viewport`
  (params (`is pop` :type Boolean))
  (locals (`temp only me` :type Boolean))
  (`|ExecutionSequence`
    (:`then_0`
      ;[1 1 1] have to collect garbage otherwise unreferenced objects in memory will mess up the logic in many parts
      (`WidgetLayoutLibrary.RemoveAllWidgets`)
      (`KismetSystemLibrary.CollectGarbage`))
    (:`then_1`
      (for (_array_element _array_index) (`self.hud class stack`)
        (bind _returnvalue (`|CreateWidget` _array_element))
        (if (== _array_index (- (`KismetArrayLibrary.Array_Length` (`self.hud class stack`)) 1))
          (set `/Game/UI/Blueprints/Main_HUD_Widget_BP.skip animation` (`local.is pop`) _returnvalue)
          (set `/Game/UI/Blueprints/Main_HUD_Widget_BP.can process input` true _returnvalue)
          (else
            (set `/Game/UI/Blueprints/Main_HUD_Widget_BP.skip animation` true _returnvalue)
            (set `/Game/UI/Blueprints/Main_HUD_Widget_BP.can process input` false _returnvalue)))
        (`UserWidget.AddToViewport` _returnvalue 0)))))

(fn `handle can control paddle`
  (params (`can control` :type Boolean))
  (bind _output_get (set `self.can control paddle` `can control`))
  (bind _maze_ref (`self.maze ref`)
    (:`then`
      (set `/Game/Blueprints/Maze/Maze_BP.can control ` _output_get _maze_ref))
    (:`else`)))

(fn `handle quit widget`
  (locals (`quit main index` :type Integer) (`tutorial count` :type Integer))
  (if (`self.manage huds`)
    (if (== (`KismetArrayLibrary.Array_Find` (`self.hud class stack`) "/Game/UI/Blueprints/Quit/Quit_Main_Widget_BP.Quit_Main_Widget_BP_C") -1)
      (`self.push hud` "/Game/UI/Blueprints/Quit/Quit_Main_Widget_BP.Quit_Main_Widget_BP_C")
      (else
        (`self.pop hud` null)))))

(fn `pop hud`
  (params (`after pop push class` :type "/Game/UI/Blueprints/Main_HUD_Widget_BP Class Reference"))
  (locals (`stack temp` :type "Array of Integer"))
  (bind _hud_class_stack (`self.hud class stack`))
  (if (`self.manage huds`)
    (`KismetArrayLibrary.Array_Remove` _hud_class_stack (- (`KismetArrayLibrary.Array_Length` _hud_class_stack) 1))
    (if (`KismetSystemLibrary.IsValidClass` `after pop push class`)
      (`KismetArrayLibrary.Array_Add` (`self.hud class stack`) `after pop push class`))
    (`self.handle adding to viewport` true)))

(fn `push hud`
  (params (`push class` :type "/Game/UI/Blueprints/Main_HUD_Widget_BP Class Reference"))
  (locals (stacktemp :type "Array of Integer"))
  (bind _hud_class_stack (`self.hud class stack`))
  (bind _output (`|GetArrayItem` _hud_class_stack (- (`KismetArrayLibrary.Array_Length` _hud_class_stack) 1)))
  (if (`self.manage huds`)
    (if (> (`KismetArrayLibrary.Array_Length` (`self.hud class stack`)) 0)
      (if (`KismetSystemLibrary.IsValidClass` _output)
        (bind _foundwidgets (`WidgetBlueprintLibrary.GetAllWidgetsOfClass` _output false))
        (for _array_element _foundwidgets
          (if (`/Game/UI/Blueprints/Main_HUD_Widget_BP.allow other hud on top` _array_element)
            (`KismetArrayLibrary.Array_Add` (`self.hud class stack`) (`local.push class`))
            (`self.handle adding to viewport` false)
            (break))))
      (else
        (`KismetArrayLibrary.Array_Add` (`self.hud class stack`) (`local.push class`))
        (`self.handle adding to viewport` false)))))

(fn `show damage on gameplay hud`
  (locals (`hud found` :type Boolean) (`gameplay hud` :type "/Game/UI/Blueprints/Gameplay/Gameplay_Main_Widget_BP Object Reference"))
  (bind _foundwidgets (`WidgetBlueprintLibrary.GetAllWidgetsOfClass` "/Game/UI/Blueprints/Gameplay/Gameplay_Main_Widget_BP.Gameplay_Main_Widget_BP_C" false))
  (for _array_element _foundwidgets
    (bind _asgameplay_main_widget_bp (cast `/Game/UI/Blueprints/Gameplay/Gameplay_Main_Widget_BP` _array_element))
    (`/Game/UI/Blueprints/Gameplay/Gameplay_Main_Widget_BP.update total damage` _asgameplay_main_widget_bp (`self.total damage`))))

(fn `UserConstructionScript`)