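; Helper Blueprint that builds a list of element-reaction damage modifiers, apparently stage effects, with descriptive text for each.
; On BeginPlay it gathers reaction names from the element-based reaction map, deduplicating through a temporary set into a name list.
; Each name gets increase and decrease entries at several fixed percentage tiers.
; A final pass writes each entry's rich-text sentence, using style tags to distinguish positive from negative values.
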(event `self.ReceiveBeginPlay`
  (`|ExecutionSequence`
    (:`then_0`
      (`self.make reaction effect list`))))

(fn `make reaction effect context`
  (for (_array_element _array_index) (`self.reaction effect list`)
    (bind (_reaction _percentage) (break `/Game/DataTypes/GamePlay/Reaction_Effect_Data_Structure` _array_element))
    (if (> _percentage 0.0)
      (`KismetArrayLibrary.Array_Set` (`self.reaction effect list`) _array_index (make `/Game/DataTypes/GamePlay/Reaction_Effect_Data_Structure` _reaction _percentage (`KismetStringLibrary.Concat_StrStr` (`KismetStringLibrary.Concat_StrStr` "<Default>" "In this stage the " "</> ") "<ReactionName>" _reaction "</>" "<Default> have increased damage by </>" "<PositiveValue>" (`KismetStringLibrary.Conv_Int64ToString` (`KismetMathLibrary.FTrunc64` _percentage)) "</>" "<Default>% .</>")))
      (else
        (bind (_reaction_2 _percentage_2) (break `/Game/DataTypes/GamePlay/Reaction_Effect_Data_Structure` _array_element))
        (`KismetArrayLibrary.Array_Set` (`self.reaction effect list`) _array_index (make `/Game/DataTypes/GamePlay/Reaction_Effect_Data_Structure` _reaction_2 _percentage (`KismetStringLibrary.Concat_StrStr` (`KismetStringLibrary.Concat_StrStr` "<Default>" "In this stage the " "</> ") "<ReactionName>" _reaction_2 "</>" "<Default> have decreased damage by </>" "<NegativeValue>" (`KismetStringLibrary.Conv_Int64ToString` (`KismetMathLibrary.FTrunc64` (* _percentage_2 -1.0))) "</>" "<Default>% .</>")))))))

(fn `make reaction effect list`
  (locals (temp :type "Set of String"))
  (`|ExecutionSequence`
    (:`then_0`
      (for _array_element (`self.element based reaction map`)
        (for _array_element_2 (`.reactionname_5_B5BEF03242F14001EC4E9AAEDAB0BB33` (break `/Game/DataTypes/GamePlay/Element_Based_Reaction_Map_Data_Structure` _array_element))
          (`BlueprintSetLibrary.Set_Add` (`local.temp`) _array_element_2))))
    (:`then_1`
      (`KismetArrayLibrary.Array_Clear` (`self.reaction name list`))
      (bind _result (`BlueprintSetLibrary.Set_ToArray` (`local.temp`)))
      (set `self.reaction name list` _result))
    (:`then_2`
      (`KismetArrayLibrary.Array_Clear` (`self.reaction effect list`))
      (for _array_element_3 (`self.reaction name list`)
        (`KismetArrayLibrary.Array_Add` (`self.reaction effect list`) (make `/Game/DataTypes/GamePlay/Reaction_Effect_Data_Structure` _array_element_3 25.0))
        (`KismetArrayLibrary.Array_Add` (`self.reaction effect list`) (make `/Game/DataTypes/GamePlay/Reaction_Effect_Data_Structure` _array_element_3 -25.0))
        (`KismetArrayLibrary.Array_Add` (`self.reaction effect list`) (make `/Game/DataTypes/GamePlay/Reaction_Effect_Data_Structure` _array_element_3 50.0))
        (`KismetArrayLibrary.Array_Add` (`self.reaction effect list`) (make `/Game/DataTypes/GamePlay/Reaction_Effect_Data_Structure` _array_element_3 -50.0))
        (`KismetArrayLibrary.Array_Add` (`self.reaction effect list`) (make `/Game/DataTypes/GamePlay/Reaction_Effect_Data_Structure` _array_element_3 75.0))
        (`KismetArrayLibrary.Array_Add` (`self.reaction effect list`) (make `/Game/DataTypes/GamePlay/Reaction_Effect_Data_Structure` _array_element_3 -75.0))))
    (:`then_3`
      (`self.make reaction effect context`))))

(fn `UserConstructionScript`)