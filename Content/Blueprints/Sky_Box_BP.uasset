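; Skybox actor that applies a configurable sky material to its static mesh and drives the look of the sky.
; It writes its power, scene brightness and star brightness variables into the Skybox_Material_Parameters material parameter collection.
; The same logic runs in the construction script for editor preview and again on BeginPlay at runtime.
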(event `self.ReceiveBeginPlay`
  (`PrimitiveComponent.SetMaterial` (`self.StaticMesh`) 0 (`self.sky material`))
  (`|ExecutionSequence`
    (:`then_0`
      (`KismetMaterialLibrary.SetScalarParameterValue` "/Game/Materials/Skybox_Material_Parameters.Skybox_Material_Parameters" "power" (`self.power`)))
    (:`then_1`
      (`KismetMaterialLibrary.SetScalarParameterValue` "/Game/Materials/Skybox_Material_Parameters.Skybox_Material_Parameters" "scene brightness" (`self.scene brightness`)))
    (:`then_2`
      (`KismetMaterialLibrary.SetScalarParameterValue` "/Game/Materials/Skybox_Material_Parameters.Skybox_Material_Parameters" "star brightness" (`self.star brightness`)))))

(fn `UserConstructionScript`
  (`PrimitiveComponent.SetMaterial` (`self.StaticMesh`) 0 (`self.sky material`))
  (`|ExecutionSequence`
    (:`then_0`
      (`KismetMaterialLibrary.SetScalarParameterValue` "/Game/Materials/Skybox_Material_Parameters.Skybox_Material_Parameters" "power" (`self.power`)))
    (:`then_1`
      (`KismetMaterialLibrary.SetScalarParameterValue` "/Game/Materials/Skybox_Material_Parameters.Skybox_Material_Parameters" "scene brightness" (`self.scene brightness`)))
    (:`then_2`
      (`KismetMaterialLibrary.SetScalarParameterValue` "/Game/Materials/Skybox_Material_Parameters.Skybox_Material_Parameters" "star brightness" (`self.star brightness`)))))