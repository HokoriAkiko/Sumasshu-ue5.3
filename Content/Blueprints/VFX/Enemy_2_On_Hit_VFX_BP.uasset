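; Short-lived hit effect actor for Enemy 2, shown as a mesh that animates and then removes itself.
; On BeginPlay it creates a dynamic material from the mesh's first slot and tints it with the element color.
; A timeline then drives the mesh scale and material opacity, and the actor destroys itself when the timeline finishes.
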(event `self.ReceiveBeginPlay`
  (bind _staticmesh (`self.StaticMesh`))
  (`|ExecutionSequence`
    (:`then_0`
      (bind _returnvalue (`PrimitiveComponent.CreateDynamicMaterialInstance` _staticmesh 0 (`PrimitiveComponent.GetMaterial` _staticmesh 0) "None"))
      (bind _output_get (set `self.dm` _returnvalue))
      (`MaterialInstanceDynamic.SetVectorParameterValue` _output_get "color" (`KismetMathLibrary.Conv_ColorToLinearColor` (`self.element color`))))
    (:`then_1`
      (bind (_direction _scale _opacity_track) (`Timeline|hit timeline`)
        (:`Update`
          (`SceneComponent.SetRelativeScale3D` (`self.StaticMesh`) (`KismetMathLibrary.Conv_DoubleToVector` _scale))
          (`MaterialInstanceDynamic.SetScalarParameterValue` (`self.dm`) "opacity" _opacity_track))
        (:`Finished`
          (`self.K2_DestroyActor`))))))

(fn `UserConstructionScript`)