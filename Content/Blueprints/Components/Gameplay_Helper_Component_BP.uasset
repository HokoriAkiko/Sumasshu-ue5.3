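; Gameplay helper component on Gameplay_GM that runs a maze-and-ball session: pause, end conditions and restart.
; It loads mode and stage from a save game to set time limit and projectile count.
; Tick ends sessions on timer, projectile count or both by mode; projectiles also report the last enemy's death.
; Ending pauses play, fades the visualizer and awards time bonuses; restart reloads the save and resets projectiles, HUD and maze.
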(event `switch to maze view`
  ;[1 1 1] call on transition
  (`PlayerController.SetViewTargetWithBlend` (`GameplayStatics.GetPlayerController` 0) (`self.maze ref`) 0.1 "VTBlend_Linear" 0.0 false))

(event `handle paddle control`
  (set `/Game/Blueprints/Maze/Maze_BP.can control ` (not (`self.Do Pause`)) (`self.maze ref`)))

(event `update volume levels`
  (params (duration :type "Float (double-precision)") (`new level` :type "Float (double-precision)"))
  (`AudioComponent.AdjustVolume` (`/Game/Blueprints/Sound/Audio_Visualizer_BP.Audio` (`self.visualizer ref`)) duration `new level` "Linear"))

(event `handle game pause`
  (params (`do pause` :type Boolean))
  (set `self.Do Pause` `do pause`)
  (`|ExecutionSequence`
    (:`then_0`
      (if (`self.Do Pause`)
        (`self.update volume levels` 0.1 0.05)
        (else
          (`self.update volume levels` 0.1 1.0))))
    (:`then_1`
      (bind _outactors (`GameplayStatics.GetAllActorsOfClass` "/Game/Blueprints/Ball/Ball_Projectile_BP.Ball_Projectile_BP_C"))
      (for _array_element _outactors
        (`/Game/Blueprints/Components/Projectile_Impulse_Component_BP.handle game pause ` (`/Game/Blueprints/Ball/Ball_Projectile_BP.Projectile_Impulse_Component_BP` _array_element))))
    (:`then_2`
      (`self.handle paddle control`))))

(event `init refs`
  (`|ExecutionSequence`
    (:`then_0`
      (bind _asgameplay_gm (cast `/Game/Blueprints/Gameplay_GM` (`self.GetOwner`)))
      (set `self.As Gameplay GM` _asgameplay_gm))
    (:`then_1`
      (bind _outactors (`GameplayStatics.GetAllActorsOfClass` "/Game/Blueprints/Sound/Audio_Visualizer_BP.Audio_Visualizer_BP_C"))
      (set `self.visualizer ref` (`|GetArrayItem` _outactors)))
    (:`then_2`
      (bind _outactors_2 (`GameplayStatics.GetAllActorsOfClass` "/Game/Blueprints/Maze/Maze_BP.Maze_BP_C"))
      (set `self.maze ref` (`|GetArrayItem` _outactors_2)))))

(event `fetch mode`
  (bind _savegame (`AsyncActionHandleSaveGame.AsyncLoadGameFromSlot` (`|GetEnumeratorNameAsString` (enumliteral `/Game/DataTypes/Save_Game_Slot_Names_ENUM` "NewEnumerator1")))
    (:`Completed`
      (bind _asgame_mode_and_stage_selected_save_game_bp (cast `/Game/Blueprints/Save_Game/Game_Mode_And_Stage_Selected_Save_Game_BP` _savegame))
      (set `self.Name Enum` (`/Game/Blueprints/Save_Game/Game_Mode_And_Stage_Selected_Save_Game_BP.name enum` _asgame_mode_and_stage_selected_save_game_bp))
      (set `self.Stage` (`/Game/Blueprints/Save_Game/Game_Mode_And_Stage_Selected_Save_Game_BP.stage` _asgame_mode_and_stage_selected_save_game_bp))
      (`self.init gameplay parameters`))))

(event `self.ReceiveBeginPlay`
  (`|ExecutionSequence`
    (:`then_0`
      (`self.init refs`))
    (:`then_1`
      (`self.fetch mode`))))

(event `self.ReceiveTick`
  (params (DeltaSeconds :type "Float (single-precision)"))
  (if (and (not (`self.Do Pause`)) (`self.gameplay session running`))
    (`|ExecutionSequence`
      (:`then_0`
        (switch `/Game/DataTypes/UI/Game_Mode_Name_ENUM` (`self.Name Enum`)
          (:`NewEnumerator1`
            _)
          (:`NewEnumerator2`
            _))
        (if (== (`self.projectile count`) 0)
          (set `self.gameplay session running` false :!label _label)
          (`self.handle session ending`)))
      (:`then_1`
        (switch `/Game/DataTypes/UI/Game_Mode_Name_ENUM` (`self.Name Enum`)
          (:`NewEnumerator0`
            _)
          (:`NewEnumerator2`
            _))
        (bind _output_get (set `self.gameplay length` (- (`self.gameplay length`) DeltaSeconds)))
        (if (< _output_get 0.0)
          (goto _label))))))

(event `handle session ending`
  (bind _visualizer_ref (`self.visualizer ref`))
  (`|ExecutionSequence`
    (:`then_0`
      (`self.handle game pause` true))
    (:`then_1`
      (`/Game/Blueprints/Sound/Audio_Visualizer_BP.handle fade out` _visualizer_ref 0.1)
      (set `/Game/Blueprints/Sound/Audio_Visualizer_BP.new amplitude` 0.0 _visualizer_ref))
    (:`then_2`
      (`self.update score based on time left`))
    (:`then_3`
      (bind _foundwidgets (`WidgetBlueprintLibrary.GetAllWidgetsOfClass` "/Game/UI/Blueprints/Gameplay/Gameplay_Main_Widget_BP.Gameplay_Main_Widget_BP_C" false))
      (for _array_element _foundwidgets
        (`/Game/UI/Blueprints/Gameplay/Gameplay_Main_Widget_BP.handle end` _array_element))
      (`KismetSystemLibrary.Delay` 3.0)
      ;[1 1 1] do not touch this , use only clear otherwise multiple instaance of challenge hud will be added to viewport
      (`/Game/Blueprints/Main_GM.clear` (`self.As Gameplay GM`) "/Game/UI/Blueprints/Challenge_Ended/Challenge_Ended_Main_HUD.Challenge_Ended_Main_HUD_C"))))

(event `on all enemies death`
  ;[1 1 1] when all enemies are dead in field then it will triger , called via ball projectile since it is the one dealing damage
  (bind _outactors (`GameplayStatics.GetAllActorsOfClass` "/Game/Blueprints/Obstacles/Enemy/Enemy_Base_BP.Enemy_Base_BP_C"))
  (if (== (`KismetArrayLibrary.Array_Length` _outactors) 1)
    (set `self.gameplay session running` false)
    (`self.handle session ending`)))

(event `handle session restart`
  (params (`reset level` :type Boolean))
  (bind _as_gameplay_gm (`self.As Gameplay GM`))
  (set `self.Reset Level` `reset level`)
  (if (not (`self.is fetching`))
    (bind _savegame (`AsyncActionHandleSaveGame.AsyncLoadGameFromSlot` (`|GetEnumeratorNameAsString` (enumliteral `/Game/DataTypes/Save_Game_Slot_Names_ENUM` "NewEnumerator1")))
      (:`then`
        (set `self.is fetching` true))
      (:`Completed`
        (set `self.is fetching` false)
        (bind _asgame_mode_and_stage_selected_save_game_bp (cast `/Game/Blueprints/Save_Game/Game_Mode_And_Stage_Selected_Save_Game_BP` _savegame))
        (bind _output_get (set `/Game/Blueprints/Gameplay_GM.Name Enum` (`/Game/Blueprints/Save_Game/Game_Mode_And_Stage_Selected_Save_Game_BP.name enum` _asgame_mode_and_stage_selected_save_game_bp) _as_gameplay_gm))
        (set `self.Name Enum` _output_get)
        (bind _output_get_2 (set `self.Stage` (`/Game/Blueprints/Save_Game/Game_Mode_And_Stage_Selected_Save_Game_BP.stage` _asgame_mode_and_stage_selected_save_game_bp)))
        (set `/Game/Blueprints/Gameplay_GM.Stage` _output_get_2 _as_gameplay_gm)
        (`|ExecutionSequence`
          (:`then_0`
            (`self.init gameplay parameters`))
          (:`then_1`
            (`self.check pending projectiles`))
          (:`then_2`
            (`self.reset gm`))
          (:`then_3`
            (`/Game/Blueprints/Sound/Audio_Visualizer_BP.reset ` (`self.visualizer ref`) (`self.Reset Level`)))
          (:`then_4`
            (`self.handle hud on session restart`)))))))

(event `reset gm`
  (`|ExecutionSequence`
    (:`then_0`
      (if (`self.Reset Level`)
        (`KismetArrayLibrary.Array_Clear` (`/Game/Blueprints/Gameplay_GM.selected elements` (`self.As Gameplay GM`)))
        (set `/Game/Blueprints/Gameplay_GM.selected mode layout index` -1 (`self.As Gameplay GM`))))
    (:`then_1`
      (bind _foundwidgets (`WidgetBlueprintLibrary.GetAllWidgetsOfClass` "/Game/UI/Blueprints/Main_HUD_Widget_BP.Main_HUD_Widget_BP_C" false))
      (for _array_element _foundwidgets
        (`/Game/UI/Blueprints/Main_HUD_Widget_BP.reset hud` _array_element)))
    (:`then_3`
      (`/Game/Blueprints/Widget_Helper_BP.reset ` (`/Game/Blueprints/Main_GM.widget helper ref` (`self.As Gameplay GM`))))
    (:`then_4`
      (`/Game/Blueprints/Gameplay_GM.populate maze` (`self.As Gameplay GM`)))))

(fn `check pending projectiles`
  ;[1 1 1] it didnt actually got hit by blast , rather its a way to skip the conditioning and directly reset the states of paddle uttons etc...
  (bind _outactors (`GameplayStatics.GetAllActorsOfClass` "/Game/Blueprints/Ball/Ball_Projectile_BP.Ball_Projectile_BP_C"))
  (for _array_element _outactors
    (`/Game/Blueprints/Ball/Ball_Projectile_BP.kill check` _array_element true)))

(fn `handle hud on session restart`
  (if (`self.Reset Level`)
    (`/Game/Blueprints/Main_GM.clear` (`self.As Gameplay GM`) "/Game/UI/Blueprints/Mode_Info/Begin_Play_Mode_Info_Main_Widget_BP.Begin_Play_Mode_Info_Main_Widget_BP_C")
    (else
      (`/Game/Blueprints/Main_GM.clear` (`self.As Gameplay GM`) "/Game/UI/Blueprints/Transition/Restart/Restart_Challenge_Transition_2.Restart_Challenge_Transition_2_C"))))

(fn `init gameplay parameters`
  (`|ExecutionSequence`
    (:`then_0`
      (set `self.gameplay length` (`KismetMathLibrary.Conv_IntToDouble` (+ (* (`self.Stage`) 10) 90))))
    (:`then_1`
      (switch `int` (`self.Stage`)
        (:`1`
          (set `self.projectile count` 4 :!label _label))
        (:`2`
          (goto _label))
        (:`3`
          (goto _label))
        (:`4`
          (set `self.projectile count` 3 :!label _label_2))
        (:`5`
          (goto _label_2))))
    (:`then_2`
      (set `/Game/Blueprints/Main_GM.total damage` 0 (`self.As Gameplay GM`)))))

(fn `update score based on time left`
  (bind _outactors (`GameplayStatics.GetAllActorsOfClass` "/Game/Blueprints/Obstacles/Enemy/Enemy_Base_BP.Enemy_Base_BP_C"))
  (if (and (== (`KismetArrayLibrary.Array_Length` _outactors) 1) (`|EnumInequality` (`self.Name Enum`) "NewEnumerator1"))
    (`/Game/Blueprints/Main_GM.calculate total damage` (`self.As Gameplay GM`) (* (`KismetMathLibrary.FTrunc` (`self.gameplay length`)) 500))))