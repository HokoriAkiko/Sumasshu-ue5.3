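; Sound handler component that applies saved volume settings and manages a stack of sounds.
; On BeginPlay it async-loads the settings save, or creates one, then sets music, UI and VFX class volumes on the main sound mix, scaled by master volume, and saves back.
; PushSound plays the new top and delay-stops the others.
; PopSound removes the top without stopping it, then restarts the new top.
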(event `self.ReceiveBeginPlay`
  (`self.fetch settings`))

(event `fetch settings`
  (bind _savegame (`AsyncActionHandleSaveGame.AsyncLoadGameFromSlot` (`|GetEnumeratorNameAsString` (enumliteral `/Game/DataTypes/Save_Game_Slot_Names_ENUM` "NewEnumerator4")))
    (:`Completed`
      (bind _assettings_saved_bp (cast `/Game/Blueprints/Save_Game/Settings_Saved_BP` _savegame)
        (:`then`
          (set `self.settings save game ref` _assettings_saved_bp))
        (:`CastFailed`
          (bind _returnvalue (`GameplayStatics.CreateSaveGameObject` "/Game/Blueprints/Save_Game/Settings_Saved_BP.Settings_Saved_BP_C"))
          (set `self.settings save game ref` _returnvalue)))
      (`self.update audio parameters`))))

(event `save settings`
  (`AsyncActionHandleSaveGame.AsyncSaveGameToSlot` (`self.settings save game ref`) (`|GetEnumeratorNameAsString` (enumliteral `/Game/DataTypes/Save_Game_Slot_Names_ENUM` "NewEnumerator4"))))

(event `update audio parameters`
  (bind _settings_save_game_ref (`self.settings save game ref`))
  (bind _settings_save_game_ref_2 (`self.settings save game ref`))
  (bind _settings_save_game_ref_3 (`self.settings save game ref`))
  (`|ExecutionSequence`
    (:`then_0`
      (`GameplayStatics.SetSoundMixClassOverride` "/Game/Blueprints/Sound/Main_Sound_Class_Mix.Main_Sound_Class_Mix" "/Game/Blueprints/Sound/Music_Sound_Class.Music_Sound_Class" (* (`/Game/Blueprints/Save_Game/Settings_Saved_BP.Master Volume` _settings_save_game_ref_2) (`/Game/Blueprints/Save_Game/Settings_Saved_BP.Music Volume` _settings_save_game_ref_2) 0.01) 1.0 0.0 false))
    (:`then_1`
      (`GameplayStatics.SetSoundMixClassOverride` "/Game/Blueprints/Sound/Main_Sound_Class_Mix.Main_Sound_Class_Mix" "/Game/Blueprints/Sound/UI_Sound_Class.UI_Sound_Class" (* (`/Game/Blueprints/Save_Game/Settings_Saved_BP.Master Volume` _settings_save_game_ref_3) (`/Game/Blueprints/Save_Game/Settings_Saved_BP.UI Volume` _settings_save_game_ref_3) 0.0025) 1.0 0.0 false))
    (:`then_2`
      (`GameplayStatics.SetSoundMixClassOverride` "/Game/Blueprints/Sound/Main_Sound_Class_Mix.Main_Sound_Class_Mix" "/Game/Blueprints/Sound/VFX_Sound_Class.VFX_Sound_Class" (* (`/Game/Blueprints/Save_Game/Settings_Saved_BP.Master Volume` _settings_save_game_ref) (`/Game/Blueprints/Save_Game/Settings_Saved_BP.VFX Volume` _settings_save_game_ref) 0.0025) 1.0 0.0 false))
    (:`then_3`
      (`GameplayStatics.PushSoundMixModifier` "/Game/Blueprints/Sound/Main_Sound_Class_Mix.Main_Sound_Class_Mix"))
    (:`then_4`
      (`self.save settings`))))

(fn `pop sound`
  (bind _stack (`self.stack`))
  (bind _returnvalue (- (`KismetArrayLibrary.Array_Length` _stack) 1))
  (bind _returnvalue_2 (`KismetArrayLibrary.Array_RemoveItem` _stack (`|GetArrayItem` _stack _returnvalue)))
  (if _returnvalue_2
    (for (_array_element _array_index) _stack
      (if (== _array_index _returnvalue)
        (`AudioComponent.Play` _array_element 0.0)
        (else
          (`AudioComponent.Stop` _array_element))))))

(fn `push sound`
  (params (sound :type "AudioComponent Object Reference"))
  (bind _stack (`self.stack`))
  (`|ExecutionSequence`
    (:`then_0`
      (`KismetArrayLibrary.Array_Add` (`self.stack`) sound))
    (:`then_1`
      (for (_array_element _array_index) _stack
        (`/Engine/EditorBlueprintResources/StandardMacros.IsValid` _array_element
          (:`Is Valid`
            (if (== _array_index (- (`KismetArrayLibrary.Array_Length` _stack) 1))
              (`AudioComponent.Play` _array_element 0.0)
              (else
                (`AudioComponent.StopDelayed` _array_element 0.5)))))))))