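; Widget_Helper_BP is a memory store that keeps string key-value pairs per widget class.
; AddInWidgetMemory finds the class entry in the WidgetMemory struct array, then updates the matching key or appends a new pair, creating the class entry if missing.
; GetValue searches the same nested arrays linearly and returns an empty string when nothing matches.
; Reset clears all stored memory.
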(fn `Add In Widget Memory`
  (params (`my class` :type "UserWidget Class Reference") (`my key` :type String) (`my value` :type String))
  (locals (`memory index` :type Integer :default -1) (`pair index` :type Integer :default -1))
  (bind (_output_widgetclass _output_pairs) (break `/Game/DataTypes/UI/Widget_Memory_Data_Structure` (`|GetArrayItem` (`self.widget memory`) (`local.memory index`))))
  (bind (_output_widgetclass_2 _output_pairs_2) (break `/Game/DataTypes/UI/Widget_Memory_Data_Structure` (`|GetArrayItem` (`self.widget memory`) (`local.memory index`))))
  (bind (_output_widgetclass_3 _output_pairs_3) (break `/Game/DataTypes/UI/Widget_Memory_Data_Structure` (`|GetArrayItem` (`self.widget memory`) (`local.memory index`))))
  (bind _string_key_value_pair_data_structure (make `/Game/DataTypes/UI/String_Key_Value_Pair_Data_Structure` (`local.my key`) (`local.my value`)))
  (`|ExecutionSequence`
    (:`then_0`
      (for (_array_element _array_index) (`self.widget memory`)
        (if (== (`local.my class`) (break `/Game/DataTypes/UI/Widget_Memory_Data_Structure` _array_element))
          (set `local.memory index` _array_index)
          (break))))
    (:`then_1`
      (if (!= (`local.memory index`) -1)
        (for (_array_element_2 _array_index_2) _output_pairs
          (if (`KismetStringLibrary.EqualEqual_StrStr` (`local.my key`) (break `/Game/DataTypes/UI/String_Key_Value_Pair_Data_Structure` _array_element_2))
            (set `local.pair index` _array_index_2)
            (break)))
        (if (== (`local.pair index`) -1)
          (`KismetArrayLibrary.Array_Add` _output_pairs_3 _string_key_value_pair_data_structure)
          (else
            (`KismetArrayLibrary.Array_Set` _output_pairs_2 (`local.pair index`) _string_key_value_pair_data_structure)))
        (else
          (`KismetArrayLibrary.Array_Add` (`self.widget memory`) (make `/Game/DataTypes/UI/Widget_Memory_Data_Structure` (`local.my class`) (`|MakeArray` (make `/Game/DataTypes/UI/String_Key_Value_Pair_Data_Structure` (`local.my key`) (`local.my value`))))))))))

(fn `get value`
  (params (`my class` :type "UserWidget Class Reference") (`my key` :type String))
  (returns (`return value` :type String))
  (locals (`class index` :type Integer :default -1))
  (bind (_output_widgetclass _output_pairs) (break `/Game/DataTypes/UI/Widget_Memory_Data_Structure` (`|GetArrayItem` (`self.widget memory`) (`local.class index`))))
  (`|ExecutionSequence`
    (:`then_0`
      (for (_array_element _array_index) (`self.widget memory`)
        (if (== (`local.my class`) (break `/Game/DataTypes/UI/Widget_Memory_Data_Structure` _array_element))
          (set `local.class index` _array_index)
          (break))))
    (:`then_1`
      (if (!= (`local.class index`) -1)
        (for _array_element_2 _output_pairs
          (if (`KismetStringLibrary.EqualEqual_StrStr` (`local.my key`) (break `/Game/DataTypes/UI/String_Key_Value_Pair_Data_Structure` _array_element_2))
            (return (`.value_5_05BCC6DA4F8A5292FCBEDD811F7521B1` (break `/Game/DataTypes/UI/String_Key_Value_Pair_Data_Structure` _array_element_2))))))
      (return ""))))

(fn `reset `
  (`KismetArrayLibrary.Array_Clear` (`self.widget memory`)))

(fn `UserConstructionScript`)