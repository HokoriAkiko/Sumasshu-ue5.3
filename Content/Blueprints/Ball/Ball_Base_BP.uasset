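; Base ball actor Blueprint that shows its assigned element's color on its meshes and effects.
; BeginPlay creates dynamic materials for Body and Outline, which a helper function tints from the ElementAssignmentComponent's selected color.
; Another function sends that color, multiplied for HDR intensity, to the motion and spawning cube VFX.
; A copy function takes element name and color from another actor's assignment component without refreshing the visuals.
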(event `self.ReceiveBeginPlay`
  (bind _body (`self.body`))
  (bind _outline (`self.outline`))
  (`|ExecutionSequence`
    (:`then_0`
      (bind _returnvalue (`PrimitiveComponent.CreateDynamicMaterialInstance` _body 0 (`PrimitiveComponent.GetMaterial` _body 0) "None"))
      (set `self.body dm` _returnvalue))
    (:`then_1`
      (bind _returnvalue_2 (`PrimitiveComponent.CreateDynamicMaterialInstance` _outline 0 (`PrimitiveComponent.GetMaterial` _outline 0) "None"))
      (set `self.outline dm` _returnvalue_2))))

(fn `Copy Element from Other Actor`
  (params (`other actor` :type "Actor Object Reference"))
  (bind _element_assignment_component (`self.Element_Assignment_Component`))
  (bind _returnvalue (`self.GetComponentByClass` (`local.other actor`) "/Game/Blueprints/Components/Element_Assignment_Component.Element_Assignment_Component_C"))
  (set `/Game/Blueprints/Components/Element_Assignment_Component.selected element name` (`/Game/Blueprints/Components/Element_Assignment_Component.selected element name` _returnvalue) _element_assignment_component)
  (set `/Game/Blueprints/Components/Element_Assignment_Component.selected element color` (`/Game/Blueprints/Components/Element_Assignment_Component.selected element color` _returnvalue) _element_assignment_component))

(fn `update ball color`
  (`|ExecutionSequence`
    (:`then_0`
      (`MaterialInstanceDynamic.SetVectorParameterValue` (`self.body dm`) "color" (`KismetMathLibrary.Conv_ColorToLinearColor` (`/Game/Blueprints/Components/Element_Assignment_Component.selected element color` (`self.Element_Assignment_Component`))))
      (`MaterialInstanceDynamic.SetVectorParameterValue` (`self.outline dm`) "color" (`KismetMathLibrary.Conv_ColorToLinearColor` (`/Game/Blueprints/Components/Element_Assignment_Component.selected element color` (`self.Element_Assignment_Component`)))))))

(fn `update vfx as per state`
  (`NiagaraComponent.SetVariableLinearColor` (`self.motion vfx`) "element_color" (* (`KismetMathLibrary.Conv_ColorToLinearColor` (`/Game/Blueprints/Components/Element_Assignment_Component.selected element color` (`self.Element_Assignment_Component`))) (struct :`R` 100.0 :`G` 100.0 :`B` 100.0 :`A` 1.0)))
  (`NiagaraComponent.SetVariableLinearColor` (`self.spawning cube vfx`) "element_color" (* (`KismetMathLibrary.Conv_ColorToLinearColor` (`/Game/Blueprints/Components/Element_Assignment_Component.selected element color` (`self.Element_Assignment_Component`))) (struct :`R` 100.0 :`G` 100.0 :`B` 100.0 :`A` 1.0))))

(fn `UserConstructionScript`)