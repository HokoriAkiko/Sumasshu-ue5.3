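; Enemy 2 is an element-colored enemy obstacle with a vertex guard, extending a parent enemy's init, hit and kill logic.
; On begin play or re-init it tints dynamic materials on its net layer and wireframe guard with the selected element color.
; One VFX handler spawns wave and status popups on elemental reactions, shatters and hides the guard once at low health, and bursts Tron cubes before destruction on kill.
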(event `/Game/Blueprints/Interface/Initialization_BPI.init again`
  (params (`selected element name` :type String) (`in memory` :type Boolean))
  (`parent.init again` `selected element name` false)
  (`self.set material as per element color` :!label _label))

(event `self.ReceiveBeginPlay`
  (`parent.ReceiveBeginPlay`)
  (goto _label))

(event `/Game/Blueprints/Interface/Kill_BPI.handle kill`
  (`parent.handle kill`)
  (`self.handle spawning of vfx` false false "" true)
  (`self.K2_DestroyActor`))

(event `/Game/Blueprints/Interface/Ball_Projectile_On_Hit_BPI.hit by projectile`
  (params (`damage configuration` :type "/Game/DataTypes/Projectile_Damage_Configuration_Data_Structure Structure") (`projectile element name` :type "String (by ref)"))
  (`parent.hit by projectile` `damage configuration` `projectile element name`)
  (`self.handle spawning of vfx` true true "Shattering Defense"))

(event `/Game/Blueprints/Interface/Blast_BPI.hit by blast`
  (params (`blast configuration` :type "/Game/DataTypes/Blast_Damage_Configuration_Data_Structure Structure"))
  (`parent.hit by blast` `blast configuration`)
  (`self.handle spawning of vfx` true true "Explosive Impact"))

(fn `handle spawning of vfx`
  (params (wave :type Boolean) (shatter :type Boolean) (status :type Text :default "NSLOCTEXT(\"[D49C66B003B987BF6E3078CDC35B02E3]\", \"E970FBFB48CB4BD6B2FD8CB360DA5B36\", \"Default Status\")") (tron :type Boolean))
  (`|ExecutionSequence`
    (:`then_0`
      (if (`local.wave`)
        (bind _net_layer (`self.net layer`)
          (:`then`
            (if (`self.reaction occured`)
              (`|SpawnActorFromClass` "/Game/Blueprints/VFX/Enemy_2_On_Hit_VFX_BP.Enemy_2_On_Hit_VFX_BP_C" (`KismetMathLibrary.MakeTransform` (`SceneComponent.K2_GetComponentLocation` _net_layer)) "Undefined" "MultiplyWithRoot" null (`/Game/Blueprints/Components/Element_Assignment_Component.selected element color` (`self.Element_Assignment_Component`)) null)))
          (:`else`))))
    (:`then_1`
      (if (`local.shatter`)
        (if (< (`self.my hp percent`) 25)
          (`/Engine/EditorBlueprintResources/StandardMacros.DoOnce` false
            (:`Completed`
              (`GameplayStatics.PlaySound2D` "/Game/Audio/cue/E2_Guard_Shatter_Cue.E2_Guard_Shatter_Cue" 1.0 1.0 0.0 null null)
              (bind _vertex_guard (`self.vertex guard`)
                (:`then`
                  (bind _element_assignment_component (`self.Element_Assignment_Component`)
                    (:`then`
                      (`|SpawnActorFromClass` "/Game/Blueprints/VFX/Enemy_2_Guard_Shatter_VFX_BP.Enemy_2_Guard_Shatter_VFX_BP_C" (`KismetMathLibrary.MakeTransform` (`SceneComponent.K2_GetComponentLocation` _vertex_guard)) "Undefined" "MultiplyWithRoot" null (`KismetMathLibrary.Conv_ColorToLinearColor` (`/Game/Blueprints/Components/Element_Assignment_Component.selected element color` _element_assignment_component)) null)
                      (bind _vertex_guard_2 (`self.vertex guard`)
                        (:`then`
                          (`SceneComponent.SetHiddenInGame` _vertex_guard_2 true true))
                        (:`else`)))
                    (:`else`)))
                (:`else`)))))))
    (:`then_2`
      (if (and (!= (`KismetStringLibrary.Len` (`KismetTextLibrary.Conv_TextToString` (`local.status`))) 0) (`self.reaction occured`))
        (bind _collider (`self.collider`)
          (:`then`
            (`|SpawnActorFromClass` "/Game/Blueprints/Hit_Status_Popup_BP.Hit_Status_Popup_BP_C" (`KismetMathLibrary.MakeTransform` (`SceneComponent.K2_GetComponentLocation` _collider)) "Undefined" "MultiplyWithRoot" null (`local.status`) null))
          (:`else`))))
    (:`then_3`
      (if (`local.tron`)
        (bind _element_assignment_component_2 (`self.Element_Assignment_Component`)
          (:`then`
            (`|SpawnActorFromClass` "/Game/Blueprints/VFX/Enemy_On_Hit_Tron_Cube_VFX_BP.Enemy_On_Hit_Tron_Cube_VFX_BP_C" (`KismetMathLibrary.MakeTransform` (`SceneComponent.K2_GetComponentLocation` (`self.vertex guard`))) "Undefined" "MultiplyWithRoot" null (`/Game/Blueprints/Components/Element_Assignment_Component.selected element color` _element_assignment_component_2) null))
          (:`else`))))))

(fn `set material as per element color`
  (bind _net_layer (`self.net layer`))
  (bind _vertex_wireframe_guard (`self.vertex wireframe guard`))
  (`|ExecutionSequence`
    (:`then_0`
      (bind _returnvalue (`PrimitiveComponent.CreateDynamicMaterialInstance` _net_layer 0 (`PrimitiveComponent.GetMaterial` _net_layer 0) "None"))
      (`MaterialInstanceDynamic.SetVectorParameterValue` _returnvalue "color" (`KismetMathLibrary.Conv_ColorToLinearColor` (`/Game/Blueprints/Components/Element_Assignment_Component.selected element color` (`self.Element_Assignment_Component`)))))
    (:`then_1`
      (bind _returnvalue_2 (`PrimitiveComponent.CreateDynamicMaterialInstance` _vertex_wireframe_guard 0 (`PrimitiveComponent.GetMaterial` _vertex_wireframe_guard 0) "None"))
      (`MaterialInstanceDynamic.SetVectorParameterValue` _returnvalue_2 "color" (`KismetMathLibrary.Conv_ColorToLinearColor` (`/Game/Blueprints/Components/Element_Assignment_Component.selected element color` (`self.Element_Assignment_Component`)))))))

(fn `UserConstructionScript`)