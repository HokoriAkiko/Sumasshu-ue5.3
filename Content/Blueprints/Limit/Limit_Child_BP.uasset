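; Limit_Child_BP is a boundary wall actor, apparently a child Blueprint, that plays a Niagara effect when hit by a projectile.
; Left, right and front wall events move the Niagara component to that side and set its facing vector parameter.
; The front wall event also sets the box size parameter, while the side events leave it unchanged.
; HitbyProjectile activates the effect with a reset.
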(event `left wall position`
  (bind _niagara (`self.Niagara`))
  (`SceneComponent.K2_SetRelativeLocation` _niagara (-200.0 100.0 0.0) false false)
  (`NiagaraComponent.SetVariableVec3` _niagara "my_facing_vector" (1.0 0.0 0.0)))

(event `right wall position`
  (bind _niagara (`self.Niagara`))
  (`SceneComponent.K2_SetRelativeLocation` _niagara (0.0 100.0 0.0) false false)
  (`NiagaraComponent.SetVariableVec3` _niagara "my_facing_vector" (1.0 0.0 0.0)))

(event `front wall position`
  (bind _niagara (`self.Niagara`))
  (`SceneComponent.K2_SetRelativeLocation` _niagara (-100.0 0.0 0.0) false false)
  (`NiagaraComponent.SetVariableVec3` _niagara "my_facing_vector" (0.0 1.0 0.0))
  (`NiagaraComponent.SetVariableVec3` _niagara "my_box_size" (200.0 1.0 200.0)))

(event `/Game/Blueprints/Interface/Ball_Projectile_On_Hit_BPI.hit by projectile`
  (`ActorComponent.Activate` (`self.Niagara`) true))

(fn `UserConstructionScript`)