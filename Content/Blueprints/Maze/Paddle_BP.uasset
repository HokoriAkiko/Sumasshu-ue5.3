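; Maze paddle that carries a selected element, shows it through color and icon, and launches a ball projectile from a placeholder.
; Element changes update the assignment component, placeholder ball, dynamic materials and VFX, fading in the icon unless InMemory is set.
; Launching hides the placeholder until the projectile dies; projectile hits spawn element-colored VFX and optional vibration.
; Paddle config loads asynchronously, is created if missing, and saves on Destroyed.
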(event `play element update animation`
  (if (not (`self.In Memory`))
    (bind (_direction _opacity_track) (`Timeline|icon timeline` :!via `PlayFromStart`)
      (:`Update`
        (`MaterialInstanceDynamic.SetScalarParameterValue` (`self.plane dm`) "opacity" _opacity_track)))))

(event `on element update`
  (params (`new element name` :type String) (`new element color` :type "Color Structure"))
  (bind _element_assignment_component (`self.Element_Assignment_Component`))
  (`|ExecutionSequence`
    (:`then_0`
      (set `/Game/Blueprints/Components/Element_Assignment_Component.selected element name` `new element name` _element_assignment_component))
    (:`then_1`
      (set `/Game/Blueprints/Components/Element_Assignment_Component.selected element color` `new element color` _element_assignment_component))
    (:`then_2`
      (bind _asball_placeholder_bp (cast `/Game/Blueprints/Ball/Ball_Placeholder_BP` (`ChildActorComponent.ChildActor` (`self.ball placeholder`))))
      (`/Game/Blueprints/Ball/Ball_Placeholder_BP.switch element` _asball_placeholder_bp))
    (:`then_3`
      (`self.update material as per element`))
    (:`then_4`
      (`self.play element update animation`))
    (:`then_5`
      (`self.update vfx as per element`))))

(event `launch ball`
  (`SceneComponent.SetHiddenInGame` (`self.ball placeholder`) true false)
  (`|SpawnActorFromClass` "/Game/Blueprints/Ball/Ball_Projectile_BP.Ball_Projectile_BP_C" (`KismetMathLibrary.MakeTransform` (`SceneComponent.K2_GetComponentLocation` (`self.ball placeholder`))) "Undefined" "MultiplyWithRoot" null null))

(event `on projectile death`
  (`SceneComponent.SetHiddenInGame` (`self.ball placeholder`) false false))

(event `/Game/Blueprints/Interface/Initialization_BPI.init again`
  (params (`selected element name` :type String) (`in memory` :type Boolean))
  (bind _element_assignment_component (`self.Element_Assignment_Component`))
  (set `self.In Memory` `in memory`)
  (`|ExecutionSequence`
    (:`then_0`
      (bind _output_get (set `/Game/Blueprints/Components/Element_Assignment_Component.selected element name` `selected element name` _element_assignment_component))
      (set `/Game/Blueprints/Components/Element_Assignment_Component.selected element color` (`BlueprintMapLibrary.Map_Find` (`/Game/Blueprints/Library/Element_Icon_Map_BFL.get element color map`) _output_get) _element_assignment_component))
    (:`then_1`
      (`self.make dynamic materials`))
    (:`then_2`
      (bind _asball_placeholder_bp (cast `/Game/Blueprints/Ball/Ball_Placeholder_BP` (`ChildActorComponent.ChildActor` (`self.ball placeholder`))))
      (`/Game/Blueprints/Ball/Ball_Placeholder_BP.switch element` _asball_placeholder_bp))
    (:`then_3`
      (`self.update material as per element`))
    (:`then_4`
      (`self.play element update animation`))
    (:`then_5`
      (`self.update vfx as per element`)
      (`ActorComponent.Activate` (`self.movement vfx`) true))))

(event `/Game/Blueprints/Interface/Ball_Projectile_On_Hit_BPI.hit by projectile`
  (params (`damage configuration` :type "/Game/DataTypes/Projectile_Damage_Configuration_Data_Structure Structure") (`projectile element name` :type "String (by ref)"))
  (`|ExecutionSequence`
    (:`then_0`
      (`|SpawnActorFromClass` "/Game/Blueprints/VFX/Paddle_On_Hit_VFX_BP.Paddle_On_Hit_VFX_BP_C" (`KismetMathLibrary.MakeTransform` (`SceneComponent.K2_GetComponentLocation` (`self.body`))) "Undefined" "MultiplyWithRoot" null (`/Game/Blueprints/Components/Element_Assignment_Component.selected element color` (`self.Element_Assignment_Component`)) null))
    (:`then_1`)
    (:`then_2`
      (bind _asmain_gm (cast `/Game/Blueprints/Main_GM` (`GameplayStatics.GetGameMode`)))
      (if (`/Game/Blueprints/Save_Game/Settings_Saved_BP.vibration` (`/Game/Blueprints/Main_GM.game settings` _asmain_gm))
        (`HokoriBPLibrary.handle_vibration`)))))

(event `fetch config`
  (bind _savegame (`AsyncActionHandleSaveGame.AsyncLoadGameFromSlot` (`|GetEnumeratorNameAsString` (enumliteral `/Game/DataTypes/Save_Game_Slot_Names_ENUM` "NewEnumerator3")))
    (:`Completed`
      (bind _aspaddle_config_save_game_bp (cast `/Game/Blueprints/Save_Game/Paddle_Config_Save_Game_BP` _savegame)
        (:`then`
          (set `self.my config` _aspaddle_config_save_game_bp))
        (:`CastFailed`
          (bind _returnvalue (`GameplayStatics.CreateSaveGameObject` "/Game/Blueprints/Save_Game/Paddle_Config_Save_Game_BP.Paddle_Config_Save_Game_BP_C"))
          (set `self.my config` _returnvalue)
          (`AsyncActionHandleSaveGame.AsyncSaveGameToSlot` (`self.my config`) (`|GetEnumeratorNameAsString` (enumliteral `/Game/DataTypes/Save_Game_Slot_Names_ENUM` "NewEnumerator3")) :!label _label))))))

(event `self.ReceiveDestroyed`
  (goto _label))

(fn `make dynamic materials`
  (bind _outline (`self.outline`))
  (bind _element_plane (`self.element plane`))
  (bind _body (`self.body`))
  (`|ExecutionSequence`
    (:`then_0`
      (bind _returnvalue (`PrimitiveComponent.CreateDynamicMaterialInstance` _body 0 (`PrimitiveComponent.GetMaterial` _body 0) "None"))
      (set `self.body dm` _returnvalue))
    (:`then_1`
      (bind _returnvalue_2 (`PrimitiveComponent.CreateDynamicMaterialInstance` _element_plane 0 (`PrimitiveComponent.GetMaterial` _element_plane 0) "None"))
      (set `self.plane dm` _returnvalue_2))
    (:`then_2`
      (bind _returnvalue_3 (`PrimitiveComponent.CreateDynamicMaterialInstance` _outline 0 (`PrimitiveComponent.GetMaterial` _outline 0) "None"))
      (set `self.outline dm` _returnvalue_3))))

(fn `update material as per element`
  (bind _element_assignment_component (`self.Element_Assignment_Component`))
  (bind _plane_dm (`self.plane dm`))
  (bind _returnvalue (`KismetMathLibrary.Conv_ColorToLinearColor` (`/Game/Blueprints/Components/Element_Assignment_Component.selected element color` _element_assignment_component)))
  (bind _returnvalue_2 (* _returnvalue (struct :`R` 5.0 :`G` 5.0 :`B` 5.0 :`A` 1.0)))
  (`|ExecutionSequence`
    (:`then_0`
      (`MaterialInstanceDynamic.SetVectorParameterValue` (`self.body dm`) "color" _returnvalue_2))
    (:`then_1`
      (`MaterialInstanceDynamic.SetVectorParameterValue` _plane_dm "color" _returnvalue)
      (`MaterialInstanceDynamic.SetTextureParameterValue` _plane_dm "icon" (`BlueprintMapLibrary.Map_Find` (`/Game/Blueprints/Components/Element_Assignment_Component.raw icon map` _element_assignment_component) (`/Game/Blueprints/Components/Element_Assignment_Component.selected element name` _element_assignment_component))))
    (:`then_2`
      (`MaterialInstanceDynamic.SetVectorParameterValue` (`self.outline dm`) "color" _returnvalue_2))))

(fn `update vfx as per element`
  (`|ExecutionSequence`
    (:`then_0`
      (`NiagaraComponent.SetVariableLinearColor` (`self.hit vfx`) "element_color" (* (`KismetMathLibrary.Conv_ColorToLinearColor` (`/Game/Blueprints/Components/Element_Assignment_Component.selected element color` (`self.Element_Assignment_Component`))) (struct :`R` 100.0 :`G` 100.0 :`B` 100.0 :`A` 1.0)))
      (`NiagaraComponent.SetVariableLinearColor` (`self.movement vfx`) "element_color" (* (`KismetMathLibrary.Conv_ColorToLinearColor` (`/Game/Blueprints/Components/Element_Assignment_Component.selected element color` (`self.Element_Assignment_Component`))) (struct :`R` 100.0 :`G` 100.0 :`B` 100.0 :`A` 1.0))))))

(fn `UserConstructionScript`)