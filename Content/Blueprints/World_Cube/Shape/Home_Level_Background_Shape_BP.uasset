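; Decorative background shape for the home level, a randomly scaled static mesh that moves vertically.
; On BeginPlay it scales the mesh by a random unit vector times a random magnitude, so proportions vary and axes can be negative.
; After a short random delay that staggers instances, a timeline plays, adding its Z track value to the mesh's current relative location each update, so the offset accumulates per frame.
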(event `self.ReceiveBeginPlay`
  (`|ExecutionSequence`
    (:`then_0`
      (`SceneComponent.SetRelativeScale3D` (`self.StaticMesh`) (* (`KismetMathLibrary.RandomUnitVector`) (`KismetMathLibrary.RandomFloatInRange` 20.0 50.0))))
    (:`then_1`
      (`KismetSystemLibrary.Delay` (`KismetMathLibrary.RandomFloatInRange` 1.0 3.0))
      (`self.handle timeline `))))

(event `handle timeline`
  (bind _staticmesh (`self.StaticMesh`))
  (bind (_direction _z_track) (`Timeline|z timeline` :!via `PlayFromStart`)
    (:`Update`
      (`SceneComponent.K2_SetRelativeLocation` _staticmesh (+ (`SceneComponent.RelativeLocation` _staticmesh) (`KismetMathLibrary.MakeVector` 0.0 0.0 _z_track)) false false))))

(fn `UserConstructionScript`)