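; Enemy obstacle Blueprint whose look follows its assigned element, extending a parent that handles init, hits and kills.
; On BeginPlay and InitAgain it tints the net, particle and stripe layers through dynamic material instances using the element color.
; Projectile hits that cause a reaction, and all blast hits, spawn element-colored particle and cube VFX plus a status popup.
; A kill spawns only the cube VFX, then destroys the actor.
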(event `/Game/Blueprints/Interface/Initialization_BPI.init again`
  (params (`selected element name` :type String) (`in memory` :type Boolean))
  (`parent.init again` `selected element name` false)
  (`self.set material as per element color` :!label _label))

(event `self.ReceiveBeginPlay`
  (`parent.ReceiveBeginPlay`)
  (goto _label))

(event `/Game/Blueprints/Interface/Kill_BPI.handle kill`
  (`parent.handle kill`)
  (`self.handle spawning of vfx` false true "")
  (`self.K2_DestroyActor`))

(event `/Game/Blueprints/Interface/Ball_Projectile_On_Hit_BPI.hit by projectile`
  (params (`damage configuration` :type "/Game/DataTypes/Projectile_Damage_Configuration_Data_Structure Structure") (`projectile element name` :type "String (by ref)"))
  (`parent.hit by projectile` `damage configuration` `projectile element name`)
  (if (`self.reaction occured`)
    (`self.handle spawning of vfx` true true "Breaking Apart")))

(event `/Game/Blueprints/Interface/Blast_BPI.hit by blast`
  (params (`blast configuration` :type "/Game/DataTypes/Blast_Damage_Configuration_Data_Structure Structure"))
  (`parent.hit by blast` `blast configuration`)
  (`self.handle spawning of vfx` true true "Explosion Impact"))

(fn `handle spawning of vfx`
  (params (particle :type Boolean :default true) (tron :type Boolean :default true) (`status text` :type Text :default "NSLOCTEXT(\"[0969638F16926FDAD25665E0275B21DF]\", \"53FBFC944925A9B67BC8FC84F90DF38F\", \"Default Status Text\")"))
  (`|ExecutionSequence`
    (:`then_0`
      (if (`local.particle`)
        (bind _element_assignment_component (`self.Element_Assignment_Component`)
          (:`then`
            (`|SpawnActorFromClass` "/Game/Blueprints/VFX/Enemy_On_Hit_Particles_VFX_BP.Enemy_On_Hit_Particles_VFX_BP_C" (`KismetMathLibrary.MakeTransform` (`SceneComponent.K2_GetComponentLocation` (`self.particles layer`))) "Undefined" "MultiplyWithRoot" null (`/Game/Blueprints/Components/Element_Assignment_Component.selected element color` _element_assignment_component) null))
          (:`else`))))
    (:`then_1`
      (if (`local.tron`)
        (bind _element_assignment_component_2 (`self.Element_Assignment_Component`)
          (:`then`
            (`|SpawnActorFromClass` "/Game/Blueprints/VFX/Enemy_On_Hit_Tron_Cube_VFX_BP.Enemy_On_Hit_Tron_Cube_VFX_BP_C" (`KismetMathLibrary.MakeTransform` (`SceneComponent.K2_GetComponentLocation` (`self.particles layer`))) "Undefined" "MultiplyWithRoot" null (`/Game/Blueprints/Components/Element_Assignment_Component.selected element color` _element_assignment_component_2) null))
          (:`else`))))
    (:`then_2`
      (if (!= (`KismetStringLibrary.Len` (`KismetTextLibrary.Conv_TextToString` (`local.status text`))) 0)
        (bind _collider (`self.collider`)
          (:`then`
            (`|SpawnActorFromClass` "/Game/Blueprints/Hit_Status_Popup_BP.Hit_Status_Popup_BP_C" (`KismetMathLibrary.MakeTransform` (`SceneComponent.K2_GetComponentLocation` _collider)) "Undefined" "MultiplyWithRoot" null (`local.status text`) null))
          (:`else`))))))

(fn `set material as per element color`
  (bind _net_layer (`self.net layer`))
  (bind _particles_layer (`self.particles layer`))
  (bind _stripe_layer (`self.stripe layer`))
  (`|ExecutionSequence`
    (:`then_0`
      (bind _returnvalue (`PrimitiveComponent.CreateDynamicMaterialInstance` _net_layer 0 (`PrimitiveComponent.GetMaterial` _net_layer 0) "None"))
      (`MaterialInstanceDynamic.SetVectorParameterValue` _returnvalue "line_color" (`KismetMathLibrary.Conv_ColorToLinearColor` (`/Game/Blueprints/Components/Element_Assignment_Component.selected element color` (`self.Element_Assignment_Component`)))))
    (:`then_1`
      (bind _returnvalue_2 (`PrimitiveComponent.CreateDynamicMaterialInstance` _particles_layer 0 (`PrimitiveComponent.GetMaterial` _particles_layer 0) "None"))
      (`MaterialInstanceDynamic.SetVectorParameterValue` _returnvalue_2 "color" (`KismetMathLibrary.Conv_ColorToLinearColor` (`/Game/Blueprints/Components/Element_Assignment_Component.selected element color` (`self.Element_Assignment_Component`)))))
    (:`then_2`
      (bind _returnvalue_3 (`PrimitiveComponent.CreateDynamicMaterialInstance` _stripe_layer 0 (`PrimitiveComponent.GetMaterial` _stripe_layer 0) "None"))
      (`MaterialInstanceDynamic.SetVectorParameterValue` _returnvalue_3 "color" (`KismetMathLibrary.Conv_ColorToLinearColor` (`/Game/Blueprints/Components/Element_Assignment_Component.selected element color` (`self.Element_Assignment_Component`)))))))

(fn `UserConstructionScript`)