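; Short-lived VFX actor for the Enemy 2 guard shatter effect, built on a cube guard static mesh.
; On BeginPlay it creates a dynamic material instance on the mesh and tints it with MyColor, the element color.
; A timeline then drives the mesh's relative scale and the material's opacity parameter, and the actor destroys itself when the timeline finishes.
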(event `self.ReceiveBeginPlay`
  (`self.set material as per element  color`)
  (bind (_direction _scale_track _opacity_track) (`Timeline|scale timeline` :!via `PlayFromStart`)
    (:`Update`
      (`|ExecutionSequence`
        (:`then_0`
          (`SceneComponent.SetRelativeScale3D` (`self.Cube_Guard_SM`) (`KismetMathLibrary.Conv_DoubleToVector` _scale_track)))
        (:`then_1`
          (`MaterialInstanceDynamic.SetScalarParameterValue` (`self.dm`) "opacity" _opacity_track))))
    (:`Finished`
      (`self.K2_DestroyActor`))))

(fn `set material as per element  color`
  (bind _cube_guard_sm (`self.Cube_Guard_SM`))
  (bind _returnvalue (`PrimitiveComponent.CreateDynamicMaterialInstance` _cube_guard_sm 0 (`PrimitiveComponent.GetMaterial` _cube_guard_sm 0) "None"))
  (bind _output_get (set `self.dm` _returnvalue))
  (`MaterialInstanceDynamic.SetVectorParameterValue` _output_get "color" (`self.my color`)))

(fn `UserConstructionScript`)