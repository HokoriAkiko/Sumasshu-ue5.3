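; Obstacle column actor that fills evenly spaced rows along Y with enemies, spaced by GapScale.
; Fresh columns roll SpawnProbability per row, spawn a random allowed Enemy_1 to Enemy_5 type and attach it with relative transforms.
; FetchColumn saves attached enemies' key, element and relative transform, letting a column be rebuilt from that layout with elements reapplied.
; Destroying the column destroys every Enemy_Base_BP in the world, not just its own.
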(event `develope column from memory`
  (params (`enemies layout` :type "Array of /Game/DataTypes/GamePlay/Enemy_Layout_Data_Structure Structure"))
  (for _array_element `enemies layout`
    (bind _return_value (`self.handle spawning using memory` _array_element))
    (`self.K2_AttachToComponent` _return_value (`self.DefaultSceneRoot`) "None" "KeepRelative" "KeepRelative" "KeepRelative" true)))

(event `develope column`
  (for _index (range 2 (+ (+ (`self.rows`) 1) 1))
    (bind _returnvalue (`self.handle spawning` (* (`self.multiplier`) _index)))
    (`/Engine/EditorBlueprintResources/StandardMacros.IsValid` _returnvalue
      (:`Is Valid`
        (`self.K2_AttachToComponent` _returnvalue (`self.DefaultSceneRoot`) "None" "KeepRelative" "KeepRelative" "KeepRelative" true)))))

(event `self.ReceiveBeginPlay`
  (set `self.multiplier` (+ (0.0 200.0 0.0) (`KismetMathLibrary.MakeVector` 0.0 (* (`self.gap scale`) 50)))))

(event `self.ReceiveDestroyed`
  (`|ExecutionSequence`
    (:`then_0`
      (bind _outactors (`GameplayStatics.GetAllActorsOfClass` "/Game/Blueprints/Obstacles/Enemy/Enemy_Base_BP.Enemy_Base_BP_C"))
      (for _array_element _outactors
        (`self.K2_DestroyActor` _array_element)))))

(fn `fetch column`
  (returns (`enemy layout` :type "Array of /Game/DataTypes/GamePlay/Enemy_Layout_Data_Structure Structure"))
  (locals (`temp enemy layout` :type "Array of /Game/DataTypes/GamePlay/Enemy_Layout_Data_Structure Structure"))
  (`|ExecutionSequence`
    (:`then_0`
      (for _array_element (`self.GetAttachedActors` true)
        (bind _asenemy_base_bp (cast `/Game/Blueprints/Obstacles/Enemy/Enemy_Base_BP` _array_element))
        (`KismetArrayLibrary.Array_Add` (`local.temp enemy layout`) (make `/Game/DataTypes/GamePlay/Enemy_Layout_Data_Structure` (`/Game/Blueprints/Obstacles/Enemy/Enemy_Base_BP.my key name` _asenemy_base_bp) (`/Game/Blueprints/Components/Element_Assignment_Component.selected element name` (`/Game/Blueprints/Obstacles/Enemy/Enemy_Base_BP.Element_Assignment_Component` _asenemy_base_bp)) (`SceneComponent.GetRelativeTransform` (`/Game/Blueprints/Actor_Main_BP.DefaultSceneRoot` _asenemy_base_bp))))))
    (:`then_1`
      (return (`local.temp enemy layout`)))))

(fn `handle spawning`
  (params (location :type "Vector Structure"))
  (returns (ReturnValue :type "Actor Object Reference"))
  (bind _obstacle_types_to_spawn_ (`self.obstacle types to spawn `))
  (if (and (> (`self.spawn probability`) (`KismetMathLibrary.RandomFloat`)) (!= (`KismetArrayLibrary.Array_Length` _obstacle_types_to_spawn_) 0))
    (switch `int` (`|GetArrayItem` _obstacle_types_to_spawn_ (`KismetMathLibrary.RandomIntegerInRange` 0 (- (`KismetArrayLibrary.Array_Length` _obstacle_types_to_spawn_) 1)))
      (:`1`
        (bind _returnvalue (`|SpawnActorFromClass` "/Game/Blueprints/Obstacles/Enemy/Enemy_1_BP.Enemy_1_BP_C" (`KismetMathLibrary.MakeTransform` (`local.location`)) "Undefined" "MultiplyWithRoot" null "E1" false null))
        (return _returnvalue))
      (:`2`
        (bind _returnvalue_2 (`|SpawnActorFromClass` "/Game/Blueprints/Obstacles/Enemy/Enemy_2_BP.Enemy_2_BP_C" (`KismetMathLibrary.MakeTransform` (`local.location`)) "Undefined" "MultiplyWithRoot" null "E2" false null))
        (return _returnvalue_2))
      (:`3`
        (bind _returnvalue_3 (`|SpawnActorFromClass` "/Game/Blueprints/Obstacles/Enemy/Enemy_3_BP.Enemy_3_BP_C" (`KismetMathLibrary.MakeTransform` (`local.location`)) "Undefined" "MultiplyWithRoot" null "E3" false null))
        (return _returnvalue_3))
      (:`4`
        (bind _returnvalue_4 (`|SpawnActorFromClass` "/Game/Blueprints/Obstacles/Enemy/Enemy_4_BP.Enemy_4_BP_C" (`KismetMathLibrary.MakeTransform` (`local.location`)) "Undefined" "MultiplyWithRoot" null "E4" false null))
        (return _returnvalue_4))
      (:`5`
        (bind _returnvalue_5 (`|SpawnActorFromClass` "/Game/Blueprints/Obstacles/Enemy/Enemy_5_BP.Enemy_5_BP_C" (`KismetMathLibrary.MakeTransform` (`local.location`)) "Undefined" "MultiplyWithRoot" null "E5" false null))
        (return _returnvalue_5)))))

(fn `handle spawning using memory`
  (params (`enemy layout` :type "/Game/DataTypes/GamePlay/Enemy_Layout_Data_Structure Structure"))
  (returns (`Return Value` :type "Actor Object Reference"))
  (bind (_enemy_layout_keyname _enemy_layout_elementname _enemy_layout_myrelativetransform) (break `/Game/DataTypes/GamePlay/Enemy_Layout_Data_Structure` (`local.enemy layout`)))
  (bind (_enemy_layout_keyname_2 _enemy_layout_elementname_2 _enemy_layout_myrelativetransform_2) (break `/Game/DataTypes/GamePlay/Enemy_Layout_Data_Structure` (`local.enemy layout`)))
  (bind (_enemy_layout_keyname_3 _enemy_layout_elementname_3 _enemy_layout_myrelativetransform_3) (break `/Game/DataTypes/GamePlay/Enemy_Layout_Data_Structure` (`local.enemy layout`)))
  (bind (_enemy_layout_keyname_4 _enemy_layout_elementname_4 _enemy_layout_myrelativetransform_4) (break `/Game/DataTypes/GamePlay/Enemy_Layout_Data_Structure` (`local.enemy layout`)))
  (bind (_enemy_layout_keyname_5 _enemy_layout_elementname_5 _enemy_layout_myrelativetransform_5) (break `/Game/DataTypes/GamePlay/Enemy_Layout_Data_Structure` (`local.enemy layout`)))
  (switch `string` `enemy layout_keyname_6_09F2CC7342595450AE2E99A689C26741`
    (:`E1`
      (bind _returnvalue (`|SpawnActorFromClass` "/Game/Blueprints/Obstacles/Enemy/Enemy_1_BP.Enemy_1_BP_C" _enemy_layout_myrelativetransform_2 "Undefined" "MultiplyWithRoot" null _enemy_layout_keyname_2 false null))
      (message `/Game/Blueprints/Interface/Initialization_BPI.init again` _returnvalue _enemy_layout_elementname_2)
      (return _returnvalue))
    (:`E2`
      (bind _returnvalue_2 (`|SpawnActorFromClass` "/Game/Blueprints/Obstacles/Enemy/Enemy_2_BP.Enemy_2_BP_C" _enemy_layout_myrelativetransform_3 "Undefined" "MultiplyWithRoot" null _enemy_layout_keyname_3 false null))
      (message `/Game/Blueprints/Interface/Initialization_BPI.init again` _returnvalue_2 _enemy_layout_elementname_3)
      (return _returnvalue_2))
    (:`E3`
      (bind _returnvalue_3 (`|SpawnActorFromClass` "/Game/Blueprints/Obstacles/Enemy/Enemy_3_BP.Enemy_3_BP_C" _enemy_layout_myrelativetransform_4 "Undefined" "MultiplyWithRoot" null _enemy_layout_keyname_4 false null))
      (message `/Game/Blueprints/Interface/Initialization_BPI.init again` _returnvalue_3 _enemy_layout_elementname_4)
      (return _returnvalue_3))
    (:`E4`
      (bind _returnvalue_4 (`|SpawnActorFromClass` "/Game/Blueprints/Obstacles/Enemy/Enemy_4_BP.Enemy_4_BP_C" _enemy_layout_myrelativetransform_5 "Undefined" "MultiplyWithRoot" null _enemy_layout_keyname_5 false null))
      (message `/Game/Blueprints/Interface/Initialization_BPI.init again` _returnvalue_4 _enemy_layout_elementname_5)
      (return _returnvalue_4))
    (:`E5`
      (bind _returnvalue_5 (`|SpawnActorFromClass` "/Game/Blueprints/Obstacles/Enemy/Enemy_5_BP.Enemy_5_BP_C" _enemy_layout_myrelativetransform "Undefined" "MultiplyWithRoot" null _enemy_layout_keyname false null))
      (message `/Game/Blueprints/Interface/Initialization_BPI.init again` _returnvalue_5 _enemy_layout_elementname)
      (return _returnvalue_5))))

(fn `UserConstructionScript`)